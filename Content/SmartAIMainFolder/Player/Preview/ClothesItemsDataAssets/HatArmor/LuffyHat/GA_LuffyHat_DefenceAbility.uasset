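; Gameplay ability for the Luffy Hat armor item that grants its owner a timed damage-reflection buff with a shield visual.
; After committing cost and cooldown, it applies GE_LuffyHat_Defence, passing duration and reflect percent through SetByCaller tags.
; It attaches a Niagara shield to the character's capsule and broadcasts the buff info through GameplayMessageSubsystem.
; The effect's removal ends the ability and destroys the shield, while a failed commit or invalid handle cancels it.
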(event `self.K2_ActivateAbility`
  (bind _returnvalue (`self.K2_CommitAbilityCost` true))
  (if _returnvalue
    (bind _returnvalue_2 (`self.K2_CommitAbilityCooldown` true))
    (if _returnvalue_2
      (`KismetSystemLibrary.PrintString` "Activate")
      (bind _returnvalue_3 (`AbilitySystemBlueprintLibrary.AssignTagSetByCallerMagnitude` (`self.MakeOutgoingGameplayEffectSpec` "/Game/SmartAIMainFolder/Player/Preview/ClothesItemsDataAssets/HatArmor/LuffyHat/GE_LuffyHat_Defence.GE_LuffyHat_Defence_C") (struct :`TagName` "Effect.Info.Duration") (`self.Duration`)))
      (bind _returnvalue_4 (`AbilitySystemBlueprintLibrary.AssignTagSetByCallerMagnitude` _returnvalue_3 (struct :`TagName` "Effect.Info.DamageReflectionPercent") (`self.ReflectPercent`)))
      (`AbilitySystemBlueprintLibrary.GetEffectContext` _returnvalue_4)
      (bind _returnvalue_5 (`self.K2_ApplyGameplayEffectSpecToOwner` _returnvalue_4))
      (bind _output_get (set `self.EffectSpec` _returnvalue_5))
      (`AbilityTask_WaitGameplayEffectRemoved.WaitForGameplayEffectRemoved` _output_get
        (:`then`
          (bind _returnvalue_6 (`NiagaraFunctionLibrary.SpawnSystemAttached` "/Game/sA_PickupSet_1/Fx/NiagaraSystems/NS_Shield_4.NS_Shield_4" (`Character.CapsuleComponent` (cast `Character` (`self.GetAvatarActorFromActorInfo`) :!pure true)) "None" (0.0 0.0 0.0) (struct) "KeepRelativeOffset"))
          (set `self.GCN` _returnvalue_6)
          (`GameplayMessageSubsystem.K2_BroadcastMessage` (subsystem `GameplayMessageSubsystem`) (struct :`TagName` "Effect.Active.Buff.DamageReflection") (make `/Game/SmartAIMainFolder/Blueprints/S_PlayerActiveGameplayEffectInfo` (`self.GetAvatarActorFromActorInfo`) (`self.EffectSpec`) (`self.ReflectPercent`) (`self.Duration`) (`self.EffectIcon`))))
        (:`OnRemoved`
          (`self.K2_EndAbility`)
          (`ActorComponent.K2_DestroyComponent` (`self.GCN`))
          (`KismetSystemLibrary.PrintString` "End"))
        (:`InvalidHandle`
          (`self.K2_CancelAbility`)))
      (else
        (`self.K2_CancelAbility` :!label _label)))
    (else
      (goto _label))))