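; Player inventory component that manages indexed main slots and type-keyed equipment slots, and handles item transfers with loot bags.
; When the Game Instance signals player spawn, it equips that instance's ItemsToEquip list.
; A gameplay message listener drives SwapSlots, which checks equipment type compatibility, then routes adds and clears by inventory type.
; Slot changes can broadcast gameplay messages; loot bag changes are only broadcast, not stored here.
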(event `self.ReceiveBeginPlay`
  (bind _asgi_base (cast `/Game/SmartAIMainFolder/Blueprints/Base/GI_Base` (`GameplayStatics.GetGameInstance`)))
  (bind _output_get (set `self.GameInstance` _asgi_base))
  (add `/Game/SmartAIMainFolder/Blueprints/Base/GI_Base.OnPlayerSpawned` _output_get (delegate `OnPlayerSpawned_Event`))
  (`KismetSystemLibrary.PrintString` "Assign")
  (bind (_asynctaskproxy _actualchannel _payload) (`|AsyncAction_ListenForGameplayMessages` (struct :`TagName` "Message.Player.Inventory.SwapSlots") "/Game/SmartAIMainFolder/Player/Blueprints/Inventory/Message/S_SmartAISwapSlotsMessage.S_SmartAISwapSlotsMessage")
    (:`OnMessageReceived`
      (bind (_slot1 _slot2) (break `/Game/SmartAIMainFolder/Player/Blueprints/Inventory/Message/S_SmartAISwapSlotsMessage` _payload))
      (`self.SwapSlots` _slot1 _slot2))))

(event `OnPlayerSpawned_Event`
  (for _array_element (`/Game/SmartAIMainFolder/Blueprints/Base/GI_Base.ItemsToEquip` (`self.GameInstance`))
    (`self.AddItemToEquippedInventory` true (`/Game/SmartAIMainFolder/Player/Preview/PDA_Equipment.Type` _array_element) _array_element)))

(fn `AddItemToEquippedInventory`
  (params (SendGameplayMessage :type Boolean) (SlotType :type "/Game/SmartAIMainFolder/Player/Preview/E_EquipmentItemType Enum" :default "NewEnumerator10") (ItemInfo :type "/Game/SmartAIMainFolder/Player/Preview/PDA_Equipment Object Reference"))
  (locals (FoundSlotInfo :type "/Game/SmartAIMainFolder/Player/Blueprints/Inventory/S_InventorySlot Structure"))
  (bind _equippedinventoryslots (`self.EquippedInventorySlots`))
  (bind (_isfree _item _index _slottype _inventorytype) (break `/Game/SmartAIMainFolder/Player/Blueprints/Inventory/S_InventorySlot` (`local.FoundSlotInfo`)))
  (bind _s_inventoryslot (make `/Game/SmartAIMainFolder/Player/Blueprints/Inventory/S_InventorySlot` false ItemInfo _index _slottype _inventorytype))
  (if (`|EnumEquality` SlotType (`/Game/SmartAIMainFolder/Player/Preview/PDA_Equipment.Type` ItemInfo))
    (set `local.FoundSlotInfo` (`BlueprintMapLibrary.Map_Find` _equippedinventoryslots SlotType))
    (`BlueprintMapLibrary.Map_Remove` _equippedinventoryslots SlotType)
    (`BlueprintMapLibrary.Map_Add` _equippedinventoryslots SlotType _s_inventoryslot)
    (if SendGameplayMessage
      (`GameplayMessageSubsystem.K2_BroadcastMessage` (subsystem `GameplayMessageSubsystem`) (`self.AddItemToEquippedInventorySlotMessageTag`) _s_inventoryslot))))

(fn `AddItemToMainInventory`
  (params (SendGameplayMessage :type Boolean) (SlotIndex :type Integer) (ItemInfo :type "/Game/SmartAIMainFolder/Player/Preview/PDA_Equipment Object Reference"))
  (bind _s_inventoryslot (make `/Game/SmartAIMainFolder/Player/Blueprints/Inventory/S_InventorySlot` false ItemInfo SlotIndex))
  (`KismetArrayLibrary.Array_Set` (`self.MainInventorySlots`) SlotIndex _s_inventoryslot)
  (if SendGameplayMessage
    (`GameplayMessageSubsystem.K2_BroadcastMessage` (subsystem `GameplayMessageSubsystem`) (`self.AddItemToInventoryMessageTag`) _s_inventoryslot)))

(fn `AddItemToSlot`
  (params (ItenInfo :type "/Game/SmartAIMainFolder/Player/Preview/PDA_Equipment Object Reference") (InventoryType :type "/Game/SmartAIMainFolder/Player/Blueprints/Inventory/E_SlotsInventoryType Enum" :default "NewEnumerator0") (SlotIndex :type Integer) (SlotType :type "/Game/SmartAIMainFolder/Player/Preview/E_EquipmentItemType Enum" :default "NewEnumerator10"))
  (switch `/Game/SmartAIMainFolder/Player/Blueprints/Inventory/E_SlotsInventoryType` InventoryType
    (:`NewEnumerator0`
      (`self.AddItemToMainInventory` true SlotIndex ItenInfo))
    (:`NewEnumerator1`
      (`self.AddItemToEquippedInventory` true SlotType ItenInfo))
    (:`NewEnumerator2`
      (`self.AddNewItemToLootBag` SlotIndex ItenInfo))))

(fn `AddNewItemToLootBag`
  (params (Index :type Integer) (Item :type "/Game/SmartAIMainFolder/Player/Preview/PDA_Equipment Object Reference"))
  (`GameplayMessageSubsystem.K2_BroadcastMessage` (subsystem `GameplayMessageSubsystem`) (struct :`TagName` "Message.LootBag.AddItem") (make `/Game/SmartAIMainFolder/Player/Blueprints/Inventory/S_InventorySlot` false Item Index "NewEnumerator10" "NewEnumerator2")))

(fn `CanSetItemToSlot`
  (params (SlotInfo :type "/Game/SmartAIMainFolder/Player/Blueprints/Inventory/S_InventorySlot Structure") (Item :type "/Game/SmartAIMainFolder/Player/Preview/PDA_Equipment Object Reference"))
  (returns (Result :type Boolean))
  (bind (_isfree _item _index _slottype _inventorytype) (break `/Game/SmartAIMainFolder/Player/Blueprints/Inventory/S_InventorySlot` SlotInfo))
  (switch `/Game/SmartAIMainFolder/Player/Blueprints/Inventory/E_SlotsInventoryType` _inventorytype
    (:`NewEnumerator0`
      _)
    (:`NewEnumerator1`
      (return (`|EnumEquality` (`/Game/SmartAIMainFolder/Player/Preview/PDA_Equipment.Type` Item) _slottype)))
    (:`NewEnumerator2`
      _))
  (return true))

(fn `CanSwap`
  (params (First :type "/Game/SmartAIMainFolder/Player/Blueprints/Inventory/S_InventorySlot Structure") (Second :type "/Game/SmartAIMainFolder/Player/Blueprints/Inventory/S_InventorySlot Structure"))
  (returns (Result :type Boolean))
  (bind (_isfree _item) (break `/Game/SmartAIMainFolder/Player/Blueprints/Inventory/S_InventorySlot` First))
  (bind (_isfree_2 _item_2) (break `/Game/SmartAIMainFolder/Player/Blueprints/Inventory/S_InventorySlot` Second))
  (if (not _isfree)
    (bind _result (`self.CanSetItemToSlot` Second _item))
    (if _result
      _
      (else
        (return false))))
  (if _isfree_2
    (return true)
    (else
      (bind _result_2 (`self.CanSetItemToSlot` First _item_2))
      (return _result_2))))

(fn `ClearSlot`
  (params (InventoryType :type "/Game/SmartAIMainFolder/Player/Blueprints/Inventory/E_SlotsInventoryType Enum" :default "NewEnumerator0") (SlotIndex :type Integer) (SlotType :type "/Game/SmartAIMainFolder/Player/Preview/E_EquipmentItemType Enum" :default "NewEnumerator10"))
  (switch `/Game/SmartAIMainFolder/Player/Blueprints/Inventory/E_SlotsInventoryType` InventoryType
    (:`NewEnumerator0`
      (`self.ClearSlotInMainInventory` SlotIndex true))
    (:`NewEnumerator1`
      (`self.ClearSlotInEquippedInventory` SlotType true))
    (:`NewEnumerator2`
      (`self.ClearSlotInLootBag` SlotIndex))))

(fn `ClearSlotInEquippedInventory`
  (params (Type :type "/Game/SmartAIMainFolder/Player/Preview/E_EquipmentItemType Enum" :default "NewEnumerator10") (SendGameplayEvent :type Boolean))
  (bind _s_inventoryslot (make `/Game/SmartAIMainFolder/Player/Blueprints/Inventory/S_InventorySlot` true null 0 Type "NewEnumerator1"))
  (`BlueprintMapLibrary.Map_Remove` (`self.EquippedInventorySlots`) Type)
  (`BlueprintMapLibrary.Map_Add` (`self.EquippedInventorySlots`) Type _s_inventoryslot)
  (if SendGameplayEvent
    (`GameplayMessageSubsystem.K2_BroadcastMessage` (subsystem `GameplayMessageSubsystem`) (`self.RemoveItemFromEquippedInventorySlotMessageTag`) _s_inventoryslot)))

(fn `ClearSlotInLootBag`
  (params (Index :type Integer))
  (`GameplayMessageSubsystem.K2_BroadcastMessage` (subsystem `GameplayMessageSubsystem`) (struct :`TagName` "Message.LootBag.ClearSlot") (make `/Game/SmartAIMainFolder/Player/Blueprints/Inventory/S_InventorySlot` true null Index "NewEnumerator10" "NewEnumerator2")))

(fn `ClearSlotInMainInventory`
  (params (Index :type Integer) (SendGameplayMessage :type Boolean))
  (bind _s_inventoryslot (make `/Game/SmartAIMainFolder/Player/Blueprints/Inventory/S_InventorySlot` true null Index))
  (`KismetArrayLibrary.Array_Set` (`self.MainInventorySlots`) Index _s_inventoryslot)
  (if SendGameplayMessage
    (`GameplayMessageSubsystem.K2_BroadcastMessage` (subsystem `GameplayMessageSubsystem`) (`self.RemoveItemFromInventoryMessageTag`) _s_inventoryslot)))

(fn `CreateMainInventorySlots`
  (`KismetArrayLibrary.Array_Clear` (`self.MainInventorySlots`))
  (for _index (range (`self.InventorySlotsAmount`))
    (`KismetArrayLibrary.Array_Add` (`self.MainInventorySlots`) (make `/Game/SmartAIMainFolder/Player/Blueprints/Inventory/S_InventorySlot` true null _index))))

(fn `GetFirstFreeSlotIndex`
  (returns (Index :type Integer))
  (for _array_element (`self.MainInventorySlots`)
    (if (break `/Game/SmartAIMainFolder/Player/Blueprints/Inventory/S_InventorySlot` _array_element)
      (return (`.Index_7_0D6D44A14C0673FC9902F6AF9C21EBB4` (break `/Game/SmartAIMainFolder/Player/Blueprints/Inventory/S_InventorySlot` _array_element))))))

(fn `SwapSlots`
  (params (First :type "/Game/SmartAIMainFolder/Player/Blueprints/Inventory/S_InventorySlot Structure") (Second :type "/Game/SmartAIMainFolder/Player/Blueprints/Inventory/S_InventorySlot Structure"))
  (bind (_isfree _item _index _slottype _inventorytype) (break `/Game/SmartAIMainFolder/Player/Blueprints/Inventory/S_InventorySlot` First))
  (bind (_isfree_2 _item_2) (break `/Game/SmartAIMainFolder/Player/Blueprints/Inventory/S_InventorySlot` Second))
  (bind (_isfree_3 _item_3 _index_2 _slottype_2 _inventorytype_2) (break `/Game/SmartAIMainFolder/Player/Blueprints/Inventory/S_InventorySlot` Second))
  (bind (_isfree_4 _item_4) (break `/Game/SmartAIMainFolder/Player/Blueprints/Inventory/S_InventorySlot` First))
  (bind _result (`self.CanSwap` First Second))
  (if _result
    (if _isfree_4
      (`self.ClearSlot` _inventorytype_2 _index_2 _slottype_2)
      (else
        (`self.AddItemToSlot` _item_4 _inventorytype_2 _index_2 _slottype_2)))
    (if _isfree_2
      (`self.ClearSlot` _inventorytype _index _slottype)
      (else
        (`self.AddItemToSlot` _item_2 _inventorytype _index _slottype)))))