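; BP_LootBag is a world loot container that holds a list of items and shows them in an inventory widget.
; On BeginPlay it records the item count and snaps to static ground below with a short downward line trace.
; Open creates WBP_LootBagInventory with the loot and a self reference.
; RemoveItem decrements the count, then at zero closes the widget, destroys the bag and triggers garbage collection.
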(event `self.ReceiveBeginPlay`
  (set `self.ItemsLeft` (`KismetArrayLibrary.Array_Length` (`self.Loot`)))
  (`self.MoveToGround`))

(fn `AddLoot`
  (params (Items :type "Array of /Game/SmartAIMainFolder/Player/Preview/PDA_Equipment Object Reference"))
  (`KismetArrayLibrary.Array_Append` (`self.Loot`) Items))

(fn `MoveToGround`
  (bind (_returnvalue_x _returnvalue_y _returnvalue_z) (`KismetMathLibrary.BreakVector` (`self.K2_GetActorLocation`)))
  (bind (_outhit _returnvalue) (`KismetSystemLibrary.LineTraceSingleForObjects` :`Start` (`self.K2_GetActorLocation`) :`End` (`KismetMathLibrary.MakeVector` _returnvalue_x _returnvalue_y (- _returnvalue_z 600.0)) :`ObjectTypes` (`|MakeArray` "ObjectTypeQuery1" :!type "EObjectTypeQuery Enum") :`DrawTime` 50.0))
  (if _returnvalue
    (`self.K2_SetActorLocation` (`.Location` (`GameplayStatics.BreakHitResult` _outhit)))))

(fn `Open`
  (bind _returnvalue (`|CreateWidget` "/Game/SmartAIMainFolder/Player/Blueprints/Inventory/LootBag/UI/WBP_LootBagInventory.WBP_LootBagInventory_C" null (`self.Loot`) self))
  (`UserWidget.AddToViewport` _returnvalue 1)
  (set `self.OpenedInventory` _returnvalue))

(fn `RemoveItem`
  (bind _result (`/Engine/EditorBlueprintResources/StandardMacros.DecrementInt` (`self.ItemsLeft`))
    (:`  `
      (if (<= _result 0)
        (`Widget.RemoveFromParent` (`self.OpenedInventory`))
        (`self.K2_DestroyActor`)
        (`KismetSystemLibrary.CollectGarbage`)))))

(fn `UserConstructionScript`)