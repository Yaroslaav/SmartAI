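; BP_HitCollider is a short-lived sphere hit volume that sizes itself from Radius and destroys itself after LifeTime.
; GetOverlappingActorsInSphere exposes the sphere's overlapping actors, filtered by class.
; The begin-overlap event does nothing; disconnected logic would call OnHit for EnemyAI-tagged actors other than the owner and destroy the collider unless MultyHit is set.
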(event `self.ReceiveBeginPlay`
  (`SphereComponent.SetSphereRadius` (`self.Sphere`) (`self.Radius`) true)
  (`KismetSystemLibrary.K2_SetTimerDelegate` (delegate `Destroy`) (`self.LifeTime`)))

(event `Destroy`
  (`self.K2_DestroyActor`))

(event `self.Sphere.OnComponentBeginOverlap`
  (params (OverlappedComponent :type "PrimitiveComponent Object Reference") (OtherActor :type "Actor Object Reference") (OtherComp :type "PrimitiveComponent Object Reference") (OtherBodyIndex :type Integer) (bFromSweep :type Boolean) (SweepResult :type "HitResult Structure (by ref)")))

(fn `GetOverlappingActorsInSphere`
  (returns (OverlappingActors :type "Array of Actor Object Reference"))
  (return (`PrimitiveComponent.GetOverlappingActors` (`self.Sphere`) (`self.Class Filter`))))

(fn `UserConstructionScript`)