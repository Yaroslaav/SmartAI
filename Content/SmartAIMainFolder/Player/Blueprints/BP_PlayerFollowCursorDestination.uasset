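; BP_PlayerFollowCursorDestination is an actor that tracks the world location under the player's cursor.
; On BeginPlay it caches the BP_TopDownController and starts a fast looping timer that moves it to each valid cursor hit.
; It listens for the FollowCursor.End gameplay message and destroys itself when that message arrives.
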(event `self.ReceiveBeginPlay`
  (`|AsyncAction_ListenForGameplayMessages` (struct :`TagName` "Message.Player.Movement.FollowCursor.End") "/Game/SmartAIMainFolder/Blueprints/S_Empty.S_Empty"
    (:`then`
      (bind _asbp_top_down_controller (cast `/Game/TopDown/Blueprints/BP_TopDownController` (`GameplayStatics.GetPlayerController` 0)))
      (set `self.PlayerController` _asbp_top_down_controller)
      (`KismetSystemLibrary.K2_SetTimerDelegate` (delegate `Move`) 0.01 true))
    (:`OnMessageReceived`
      (`self.K2_DestroyActor`))))

(event `Move`
  (bind (_hit _location) (`/Game/TopDown/Blueprints/BP_TopDownController.Get Location Under Cursor` (`self.PlayerController`)))
  (if _hit
    (`self.K2_SetActorLocation` _location)))

(fn `UserConstructionScript`)