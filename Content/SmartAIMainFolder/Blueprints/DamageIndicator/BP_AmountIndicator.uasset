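; Floating damage number actor that shows a damage amount in a widget, drifts away, then removes itself.
; On BeginPlay it passes the amount as text and a color to its WBP_FloatingDamageIndicator widget and starts it.
; A Move timeline lerps the actor's relative location from zero to an offset shifted by a random amount, then destroys the actor when finished.
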(event `self.ReceiveBeginPlay`
  (bind (_randomize_x _randomize_y) (`KismetMathLibrary.BreakVector2D` (`self.Randomize`)))
  (bind _aswbp_floating_damage_indicator (cast `/Game/SmartAIMainFolder/UI/Widgets/Game/WBP_FloatingDamageIndicator` (`WidgetComponent.GetWidget` (`self.Widget`))))
  (`/Game/SmartAIMainFolder/UI/Widgets/Game/WBP_FloatingDamageIndicator.SetInfoAndStart` _aswbp_floating_damage_indicator (`KismetTextLibrary.Conv_DoubleToText` (`self.DamageAmount`) "HalfToEven") (`self.Specified Color`))
  (set `self.EndPos` (+ (`self.MovingOffset`) (`KismetMathLibrary.RandomFloatInRange` _randomize_x _randomize_y)))
  (bind (_direction _movetrack) (`Timeline|Move`)
    (:`Update`
      (`self.K2_SetActorRelativeLocation` (`KismetMathLibrary.VLerp` (0.0 0.0 0.0) (`self.EndPos`) _movetrack)))
    (:`Finished`
      (`self.K2_DestroyActor`))))

(fn `UserConstructionScript`)