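; BP_EnemyAI_Range is an enemy AI character that, despite its Range name, fights with a sword.
; Attack, wield and sheath events play montages, whose notifies spawn BP_Sword onto the hand socket or destroy it.
; Completed or interrupted montages both fire end dispatchers, with wield and sheath also updating IsWieldingSword.
; Functions supply attack and defend radii, expose the patrol route, and map movement states to walk speed.
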(event `self.ReceiveBeginPlay`)

(event `Attack`
  (`|PlayMontage` (`self.Mesh`) "/Game/SmartAIMainFolder/Animations/Montages/StableSwordOutwardSlash_UE_Montage.StableSwordOutwardSlash_UE_Montage"
    (:`OnCompleted`
      _)
    (:`OnInterrupted`
      _))
  (`self.OnAttackEnd`))

(event `WieldSword`
  (bind _notifyname (`|PlayMontage` (`self.Mesh`) "/Game/SmartAIMainFolder/Animations/Montages/WithdrawingSword_UE_Montage.WithdrawingSword_UE_Montage")
    (:`OnCompleted`
      (set `self.IsWieldingSword` true :!label _label)
      (`self.OnWeaponWithdrawEnd`))
    (:`OnInterrupted`
      (goto _label))
    (:`OnNotifyBegin`
      (switch `name` _notifyname
        (:`HoldSword`
          (bind _returnvalue (`|SpawnActorFromClass` "/Game/SmartAIMainFolder/Weapons/BP_Sword.BP_Sword_C" (`self.GetTransform`) "Undefined" "MultiplyWithRoot" self null))
          (bind _output_get (set `self.EquipedWeapon` _returnvalue))
          (`self.K2_AttachToComponent` _output_get (`self.Mesh`) "hand_r_sword_socket" "SnapToTarget" "SnapToTarget" "SnapToTarget" true))))))

(event `SheethSword`
  (bind _notifyname (`|PlayMontage` (`self.Mesh`) "/Game/SmartAIMainFolder/Animations/Montages/SheathingSword_UE_Montage.SheathingSword_UE_Montage")
    (:`OnCompleted`
      (set `self.IsWieldingSword` false :!label _label_2)
      (`self.OnWeaponSheathingEnd`))
    (:`OnInterrupted`
      (goto _label_2))
    (:`OnNotifyBegin`
      (switch `name` _notifyname
        (:`DropSword`
          (`self.K2_DestroyActor` (`self.EquipedWeapon`)))))))

(fn `GetIdealRange`
  (returns (AttackRadius :type "Float (double-precision)") (DefendRadius :type "Float (double-precision)"))
  (return 100.0 400.0))

(fn `GetPatrolRoute`
  (returns (PatrolRoute :type "/Game/SmartAIMainFolder/Enemy/AI/BP_PatrolRoute Object Reference"))
  (return (`self.PatrolRoute`)))

(fn `SetMovementSpeed`
  (params (Speed :type "/Game/SmartAIMainFolder/Enemy/Enums/E_MovementSpeed Enum" :default "NewEnumerator0"))
  (returns (SpeedValue :type "Float (double-precision)"))
  (bind _output_get (set `CharacterMovementComponent.MaxWalkSpeed` (select `/Game/SmartAIMainFolder/Enemy/Enums/E_MovementSpeed` Speed :`NewEnumerator1` 100.0 :`NewEnumerator2` 300.0 :`NewEnumerator3` 600.0 :!type "Float (single-precision)") (`self.CharacterMovement`)))
  (return _output_get))

(fn `UserConstructionScript`)