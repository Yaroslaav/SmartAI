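; Melee enemy AI character that draws and sheathes a sword, extending a parent enemy class.
; Equip and unequip play montages whose notifies spawn the hand-socketed sword and grant its abilities, or remove those abilities and destroy it.
; Montage completion or interruption updates the wielding flag and signals listeners.
; Attack and Heal are empty, CalculateDamage returns zero, and an older slash-and-damage chain is left unconnected.
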(event `self.ReceiveBeginPlay`
  (`parent.ReceiveBeginPlay`))

(event `/Game/SmartAIMainFolder/Blueprints/EnemyAi/BPI_Fighter.Attack`)

(event `/Game/SmartAIMainFolder/Blueprints/EnemyAi/BPI_Fighter.EquipWeapon`
  (params (Info :type "/Game/SmartAIMainFolder/Player/Preview/PDA_Equipment Object Reference"))
  (bind _notifyname (`|PlayMontage` (`self.Mesh`) "/Game/SmartAIMainFolder/Animations/Montages/WithdrawingSword_UE_Montage.WithdrawingSword_UE_Montage")
    (:`OnCompleted`
      (set `self.IsWieldingWeapon` true :!label _label)
      (`self.OnWeaponEqiupped`))
    (:`OnInterrupted`
      (goto _label))
    (:`OnNotifyBegin`
      (switch `name` _notifyname
        (:`HoldSword`
          (bind _returnvalue (`|SpawnActorFromClass` "/Game/SmartAIMainFolder/Weapons/BP_Weapon_Sword.BP_Weapon_Sword_C" (`self.GetTransform`) "Undefined" "MultiplyWithRoot" self null))
          (bind _output_get (set `self.WeaponActor` _returnvalue))
          (`self.K2_AttachToComponent` _output_get (`self.Mesh`) "hand_r_sword_socket" "SnapToTarget" "SnapToTarget" "SnapToTarget" true)
          (bind _gameplayabilitiesspecs (`self.GiveAbilities` (`/Game/SmartAIMainFolder/Weapons/BP_Weapon_Base.Abilities` (`self.WeaponActor`))))
          (`/Game/SmartAIMainFolder/Weapons/BP_Weapon_Base.SetGivenAbilitiesSpecs` (`self.WeaponActor`) _gameplayabilitiesspecs))))))

(event `/Game/SmartAIMainFolder/Blueprints/EnemyAi/BPI_Fighter.UnequipWeapon`
  (bind _notifyname (`|PlayMontage` (`self.Mesh`) "/Game/SmartAIMainFolder/Animations/Montages/SheathingSword_UE_Montage.SheathingSword_UE_Montage")
    (:`OnCompleted`
      (set `self.IsWieldingWeapon` false :!label _label_2)
      (`self.OnWeaponUnequipped`))
    (:`OnInterrupted`
      (goto _label_2))
    (:`OnNotifyBegin`
      (switch `name` _notifyname
        (:`DropSword`
          (`self.RemoveAbilites` (`/Game/SmartAIMainFolder/Weapons/BP_Weapon_Base.AbilitiesSpecs` (`self.WeaponActor`)))
          (`self.K2_DestroyActor` (`self.WeaponActor`)))))))

(event `/Game/SmartAIMainFolder/Blueprints/EnemyAi/BPI_Fighter.Heal`
  (params (HealPercentage :type "Float (double-precision)")))

(fn `CalculateDamage`
  (returns (Damage :type "Float (double-precision)"))
  (return 0.0))

(fn `UserConstructionScript`
  (`parent.UserConstructionScript`))