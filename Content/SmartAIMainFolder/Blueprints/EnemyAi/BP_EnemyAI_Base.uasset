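; Base enemy AI character that uses the Gameplay Ability System and serves combat, patrol and movement-speed queries.
; BeginPlay caches its AI controller, grants default abilities and listens for attribute changes, which either set it attacking the player or kill it, dropping a loot bag.
; A gameplay message listener shows its decal while the player targets it.
; AnyDamage and Heal adjust a separate Health float that never calls Die.
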(event `self.ReceiveBeginPlay`
  (bind _asbp_enemy_ai_controller_base (cast `/Game/SmartAIMainFolder/Blueprints/EnemyAi/BP_EnemyAI_Controller_Base` (`AIBlueprintHelperLibrary.GetAIController` self)))
  (set `self.AIController` _asbp_enemy_ai_controller_base)
  (`self.GiveAbilities` (`self.DefaultAbilities`))
  (bind (_asynctaskproxy _attribute _newvalue) (`AsyncTaskAttributeChanged.ListenForAttributeChange` (`self.AbilitySystemComponent`) (struct :`AttributeName` "Health" :`Attribute` "/Script/SmartAI.SmartAIHealthSet:Health" :`AttributeOwner` "/Script/CoreUObject.Class'/Script/SmartAI.SmartAIHealthSet'"))
    (:`then`
      (bind (_asynctaskproxy_2 _actualchannel _payload) (`|AsyncAction_ListenForGameplayMessages` (struct :`TagName` "Message.Player.SelectTarget") "/Game/SmartAIMainFolder/MessageSS/Structs/S_PlayerSelectTarget.S_PlayerSelectTarget")
        (:`then`
          (`SceneComponent.SetVisibility` (`self.Decal`) false false))
        (:`OnMessageReceived`
          (`SceneComponent.SetVisibility` (`self.Decal`) (== (`.NewTarget_5_BA0991A7407C8EAA2BFCDEB131601BE0` (break `/Game/SmartAIMainFolder/MessageSS/Structs/S_PlayerSelectTarget` _payload)) self) false))))
    (:`OnAttributeChanged`
      (`self.CheckHealth` _newvalue))))

(event `self.ReceiveTick`
  (params (DeltaSeconds :type "Float (single-precision)")))

(event `self.ReceiveAnyDamage`
  (params (Damage :type "Float (single-precision)") (DamageType :type "DamageType Object Reference") (InstigatedBy :type "Controller Object Reference") (DamageCauser :type "Actor Object Reference"))
  (bind _output_get (set `self.Health` (`KismetMathLibrary.FClamp` (- (`self.Health`) Damage) 0.0 (`self.MaxHealth`))))
  (if (<= _output_get 0.0)
    (set `self.IsDead` true)))

(event `/Game/SmartAIMainFolder/Blueprints/EnemyAi/BPI_Fighter.Heal`
  (params (HealPercentage :type "Float (double-precision)"))
  (set `self.Health` (`KismetMathLibrary.FClamp` (+ (* HealPercentage (`self.MaxHealth`)) (`self.Health`)) 0.0 (`self.MaxHealth`))))

(fn `CheckHealth`
  (params (NewValue :type "Float (single-precision)"))
  (if (<= NewValue 0.0)
    (`self.Die`)
    (else
      (`/Game/SmartAIMainFolder/Blueprints/EnemyAi/BP_EnemyAI_Controller_Base.SetStateAsAttacking` (`self.AIController`) (`/Game/TopDown/Blueprints/BP_TopDownController.OwningBPPlayer` (cast `/Game/TopDown/Blueprints/BP_TopDownController` (`GameplayStatics.GetPlayerController` 0) :!pure true))))))

(fn `Die`
  (bind _weaponactor (`self.WeaponActor`))
  (`self.K2_DestroyActor`)
  (`|SpawnActorFromClass` "/Game/SmartAIMainFolder/Player/Blueprints/Inventory/LootBag/BP_LootBag.BP_LootBag_C" (`self.GetTransform`) "AlwaysSpawn" "MultiplyWithRoot" null (`|MakeArray` "/Game/SmartAIMainFolder/Equipment/DA_Bloodletter.DA_Bloodletter" :!type "/Game/SmartAIMainFolder/Player/Preview/PDA_Equipment Object Reference") null)
  (`/Engine/EditorBlueprintResources/StandardMacros.IsValid` _weaponactor
    (:`Is Valid`
      (`self.K2_DestroyActor` _weaponactor))))

(fn `GetCharacterInfo`
  (returns (Info :type "/Game/SmartAIMainFolder/Blueprints/S_CharacterInfo Structure"))
  (return))

(fn `GetCurrentHealth`
  (returns (NewParam :type "Float (double-precision)"))
  (return (`self.Health`)))

(fn `GetGrantedAbilitySpec`
  (params (Ability :type "GameplayAbility Class Reference"))
  (returns (SpecHandle :type "GameplayAbilitySpecHandle Structure") (Found :type Boolean))
  (bind (_value _returnvalue) (`BlueprintMapLibrary.Map_Find` (`self.GrantedAbilitiesSpecs`) Ability))
  (return _value _returnvalue))

(fn `GetHeight`
  (returns (Height :type "Float (double-precision)"))
  (return (* (`CapsuleComponent.CapsuleHalfHeight` (`self.CapsuleComponent`)) 2.0)))

(fn `GetIdealRange`
  (returns (AttackRadius :type "Float (double-precision)") (DefendRadius :type "Float (double-precision)"))
  (return 100.0 400.0))

(fn `GetLastPointOfInterest`
  (returns (Point :type "Vector Structure"))
  (return (0.0 0.0 0.0)))

(fn `GetMaxHealth`
  (returns (NewParam :type "Float (double-precision)"))
  (return (`self.MaxHealth`)))

(fn `GetPatrolRoute`
  (returns (PatrolRoute :type "/Game/SmartAIMainFolder/Enemy/AI/BP_PatrolRoute Object Reference"))
  (return (`self.PatrolRoute`)))

(fn `GetSkeletalMesh`
  (returns (SkeletalMeshComponent :type "SkeletalMeshComponent Object Reference"))
  (return null))

(fn `GetTarget`
  (returns (TargetActor :type "Actor Object Reference"))
  (return (`/Game/SmartAIMainFolder/Blueprints/EnemyAi/BP_EnemyAI_Controller_Base.AttackTarget` (`self.AIController`))))

(fn `GiveAbilities`
  (params (Abilities :type "Array of GameplayAbility Class Reference"))
  (returns (GameplayAbilitiesSpecs :type "Array of GameplayAbilitySpecHandle Structure"))
  (locals (AbilitiesSpecs :type "Array of GameplayAbilitySpecHandle Structure"))
  (bind _abilitiesspecs (`local.AbilitiesSpecs`))
  (for _array_element Abilities
    (bind _returnvalue (`AbilitySystemComponent.K2_GiveAbility` (`self.AbilitySystemComponent`) _array_element 0 -1))
    (`BlueprintMapLibrary.Map_Add` (`self.GrantedAbilitiesSpecs`) _array_element _returnvalue)
    (`KismetArrayLibrary.Array_Add` _abilitiesspecs _returnvalue)
    (return _abilitiesspecs)))

(fn `GrantAbilities`
  (params (Abilities :type "Array of GameplayAbility Class Reference (by ref)"))
  (returns (Specs :type "Array of GameplayAbilitySpecHandle Structure"))
  (return))

(fn `GrantAbility`
  (params (Ability :type "GameplayAbility Class Reference"))
  (returns (Spec :type "GameplayAbilitySpecHandle Structure"))
  (return))

(fn `RemoveAbilites`
  (params (Specs :type "Array of GameplayAbilitySpecHandle Structure (by ref)"))
  (for _array_element Specs
    (`AbilitySystemComponent.ClearAbility` (`self.AbilitySystemComponent`) _array_element)))

(fn `SetMovementSpeed`
  (params (Speed :type "/Game/SmartAIMainFolder/Enemy/Enums/E_MovementSpeed Enum" :default "NewEnumerator0"))
  (returns (SpeedValue :type "Float (double-precision)"))
  (bind _output_get (set `CharacterMovementComponent.MaxWalkSpeed` (select `/Game/SmartAIMainFolder/Enemy/Enums/E_MovementSpeed` Speed :`NewEnumerator1` 100.0 :`NewEnumerator2` 300.0 :`NewEnumerator3` 600.0 :!type "Float (single-precision)") (`self.CharacterMovement`)))
  (return _output_get))

(fn `UserConstructionScript`)