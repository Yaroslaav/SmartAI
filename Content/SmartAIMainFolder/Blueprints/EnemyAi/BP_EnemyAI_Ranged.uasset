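; Ranged enemy AI character, a child of a shared enemy base, that fights with a rifle.
; On BeginPlay it spawns the rifle and attaches it to a hand socket.
; Attack plays a firing montage whose notify applies fixed damage directly to the current target, with no trace or projectile, then signals attack end.
; It also handles percentage-based healing and supplies movement speeds per state and ideal attack and defend ranges.
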(event `self.ReceiveBeginPlay`
  (`parent.ReceiveBeginPlay`)
  (`/Game/SmartAIMainFolder/Blueprints/EnemyAi/BPI_Fighter.EquipWeapon` null))

(event `/Game/SmartAIMainFolder/Blueprints/EnemyAi/BPI_Fighter.EquipWeapon`
  (params (Info :type "/Game/SmartAIMainFolder/Player/Preview/PDA_Equipment Object Reference"))
  (bind _returnvalue (`|SpawnActorFromClass` "/Game/SmartAIMainFolder/Weapons/BP_Weapon_Rifle.BP_Weapon_Rifle_C" (`KismetMathLibrary.MakeTransform` (0.0 0.0 0.0)) "Undefined" "MultiplyWithRoot" null null))
  (bind _output_get (set `self.WeaponActor` _returnvalue))
  (`self.K2_AttachToComponent` _output_get (`self.Mesh`) "hand_r_rifle_socket" "KeepRelative" "KeepRelative" "KeepRelative" true)
  (set `self.IsWieldingWeapon` true)
  (`self.OnWeaponEqiupped`))

(event `/Game/SmartAIMainFolder/Blueprints/EnemyAi/BPI_Fighter.Attack`
  (bind _notifyname (`|PlayMontage` (`self.Mesh`) "/Game/Characters/Mannequins/Animations/Quinn/FiringRifle_UE_Montage.FiringRifle_UE_Montage")
    (:`OnCompleted`
      (`self.OnAttackEnd` :!label _label))
    (:`OnInterrupted`
      (goto _label))
    (:`OnNotifyBegin`
      (switch `name` _notifyname
        (:`Fire`
          (bind _targetactor (`/Game/SmartAIMainFolder/Blueprints/EnemyAi/BPI_Fighter.GetTarget`))
          (`GameplayStatics.ApplyDamage` _targetactor 20.0 null self))))))

(event `/Game/SmartAIMainFolder/Blueprints/EnemyAi/BPI_Fighter.Heal`
  (params (HealPercentage :type "Float (double-precision)"))
  (set `self.Health` (`KismetMathLibrary.FClamp` (+ (* HealPercentage (`self.MaxHealth`)) (`self.Health`)) 0.0 (`self.MaxHealth`)))
  (`self.OnFullyHealed`))

(fn `GetIdealRange`
  (returns (AttackRadius :type "Float (double-precision)") (DefendRadius :type "Float (double-precision)"))
  (return 600.0 600.0))

(fn `SetMovementSpeed`
  (params (Speed :type "/Game/SmartAIMainFolder/Enemy/Enums/E_MovementSpeed Enum" :default "NewEnumerator0"))
  (returns (SpeedValue :type "Float (double-precision)"))
  (bind _output_get (set `CharacterMovementComponent.MaxWalkSpeed` (select `/Game/SmartAIMainFolder/Enemy/Enums/E_MovementSpeed` Speed :`NewEnumerator1` 200.0 :`NewEnumerator2` 300.0 :`NewEnumerator3` 600.0 :!type "Float (single-precision)") (`self.CharacterMovement`)))
  (return _output_get))

(fn `UserConstructionScript`
  (`parent.UserConstructionScript`))