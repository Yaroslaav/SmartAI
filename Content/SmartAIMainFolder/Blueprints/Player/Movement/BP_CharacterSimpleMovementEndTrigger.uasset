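; Destination trigger that ends the player's simple movement in the top-down controller.
; On BeginPlay it scales its Cube horizontally by CompleteSize with a fixed height to form the overlap volume.
; When the referenced Player overlaps the cube, it calls EndMovement on that player's BP_TopDownController, then destroys itself.
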(event `self.ReceiveBeginPlay`
  (bind _completesize (`self.CompleteSize`))
  (`SceneComponent.SetRelativeScale3D` (`self.Cube`) (`KismetMathLibrary.MakeVector` _completesize _completesize 10.0)))

(event `self.Cube.OnComponentBeginOverlap`
  (params (OverlappedComponent :type "PrimitiveComponent Object Reference") (OtherActor :type "Actor Object Reference") (OtherComp :type "PrimitiveComponent Object Reference") (OtherBodyIndex :type Integer) (bFromSweep :type Boolean) (SweepResult :type "HitResult Structure (by ref)"))
  (bind _player (`self.Player`))
  (if (== OtherActor _player)
    (bind _asbp_top_down_controller (cast `/Game/TopDown/Blueprints/BP_TopDownController` (`Pawn.GetController` _player)))
    (`/Game/TopDown/Blueprints/BP_TopDownController.EndMovement` _asbp_top_down_controller)
    (`self.K2_DestroyActor`)))

(fn `UserConstructionScript`)