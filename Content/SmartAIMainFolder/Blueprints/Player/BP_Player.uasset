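; BP_Player is the player Blueprint, using the Gameplay Ability System for mana and abilities such as Dash.
; BeginPlay grants default abilities, caches the mana attribute set and applies the mana regeneration effect.
; Debug-style keys stimulate enemy AI: F makes a noise with a sound, X reports and applies damage to a found enemy.
; Helpers clamp spring-arm camera zoom and activate Dash, while Attack only prints an attribute value labelled mana.
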(event `self.ReceiveBeginPlay`
  (`parent.ReceiveBeginPlay`)
  (`self.AddAbilities` (`self.DefaultAbilities`))
  (bind _returnvalue (`AbilitySystemComponent.GetAttributeSet` (`self.AbilitySystemComponent`) "/Script/SmartAI.SmartAIManaSet"))
  (bind _assmart_aimana_set (cast `SmartAIManaSet` _returnvalue))
  (set `self.ManaAttributeSet` _assmart_aimana_set)
  (`AbilitySystemComponent.BP_ApplyGameplayEffectToSelf` :`self` (`self.AbilitySystemComponent`) :`GameplayEffectClass` "/Game/SmartAIMainFolder/GAS/Effects/ManaBase/GE_RegenMana.GE_RegenMana_C"))

(event `Key|F`
  (params (Key :type "Key Structure"))
  (bind _returnvalue (`self.K2_GetActorLocation`))
  (:`Pressed`
    (`self.MakeNoise` 1.0 self _returnvalue)
    (`GameplayStatics.PlaySoundAtLocation` "/Game/Sounds/pop2.pop2" _returnvalue (struct) 1.0 1.0 0.0 null null null null)))

(event `Key|X`
  (params (Key :type "Key Structure"))
  (:`Pressed`
    (`KismetSystemLibrary.PrintString` "Hello")
    (bind _returnvalue (`GameplayStatics.GetActorOfClass` "/Game/SmartAIMainFolder/Blueprints/EnemyAi/BP_EnemyAI_Base.BP_EnemyAI_Base_C"))
    (`AISense_Damage.ReportDamageEvent` _returnvalue self 10.0 (`self.K2_GetActorLocation`))
    (`GameplayStatics.ApplyDamage` _returnvalue 20.0 null self)))

(fn `AddAbilities`
  (params (Abilities :type "Array of GameplayAbility Class Reference"))
  (for _array_element Abilities
    (`AbilitySystemComponent.K2_GiveAbility` (`self.AbilitySystemComponent`) _array_element 0 -1)))

(fn `Attack`
  (`KismetSystemLibrary.PrintString` (`KismetStringLibrary.Concat_StrStr` "Mana - " (`KismetStringLibrary.Conv_DoubleToString` (`.ReturnValue` (`AbilitySystemBlueprintLibrary.GetFloatAttributeFromAbilitySystemComponent` (`AbilitySystemBlueprintLibrary.GetAbilitySystemComponent` null) (struct :`AttributeName` "Mana" :`Attribute` "/Script/SmartAI.SmartAIHealthSet:Mana" :`AttributeOwner` "/Script/CoreUObject.Class'/Script/SmartAI.SmartAIHealthSet'")))))))

(fn `ChangeCameraSpringArmLength`
  (params (Amount :type "Float (double-precision)"))
  (set `SpringArmComponent.TargetArmLength` (`KismetMathLibrary.FClamp` (+ (`SpringArmComponent.TargetArmLength` (`self.SpringArm`)) Amount) (`self.MinSpringArmLength`) (`self.MaxSpringArmLength`)) (`self.SpringArm`)))

(fn `Dash`
  (`AbilitySystemComponent.TryActivateAbilityByClass` (`self.AbilitySystemComponent`) "/Game/SmartAIMainFolder/GAS/Abilities/GA_Dash.GA_Dash_C" true))

(fn `UserConstructionScript`)