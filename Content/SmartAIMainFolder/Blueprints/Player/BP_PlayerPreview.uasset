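; BP_PlayerPreview is a player preview actor for the main menu that displays the clothing items selected there.
; On BeginPlay it binds to the clothes-select event on GSB_MainMenu and caches the GI_Base game instance.
; PutOn maps the item type to the head, chest or foot mesh component, applies the item's mesh and relative transform, then passes the item to the game instance through SetClothes.
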(event `self.ReceiveBeginPlay`
  (bind _asgsb_main_menu (cast `/Game/SmartAIMainFolder/Blueprints/Base/MainMenu/GSB_MainMenu` (`GameplayStatics.GetGameState`)))
  (bind _output_get (set `self.GameState` _asgsb_main_menu))
  (add `/Game/SmartAIMainFolder/Blueprints/Base/MainMenu/GSB_MainMenu.OnClothesItemSelect` _output_get (delegate `OnClothesItemSelect_Event`))
  (bind _asgi_base (cast `/Game/SmartAIMainFolder/Blueprints/Base/GI_Base` (`GameplayStatics.GetGameInstance`)))
  (set `self.GIBase` _asgi_base))

(event `OnClothesItemSelect_Event`
  (params (ItemInfo :type "/Game/SmartAIMainFolder/Player/Preview/PDA_ClothesItem Object Reference"))
  (`self.PutOn` ItemInfo))

(fn `PutOn`
  (params (ClothesInfo :type "/Game/SmartAIMainFolder/Player/Preview/PDA_ClothesItem Object Reference"))
  (locals (CurMesh :type "SkeletalMeshComponent Object Reference"))
  (switch `/Game/SmartAIMainFolder/Player/Preview/E_ClothesItemType` (`/Game/SmartAIMainFolder/Player/Preview/PDA_ClothesItem.Type` ClothesInfo)
    (:`NewEnumerator0`
      (set `local.CurMesh` (`self.Head`)))
    (:`NewEnumerator1`
      (set `local.CurMesh` (`self.Chest`)))
    (:`NewEnumerator2`
      (set `local.CurMesh` (`self.FootL`)))
    (:`NewEnumerator3`
      (set `local.CurMesh` (`self.FootR`))))
  (`SkeletalMeshComponent.SetSkeletalMeshAsset` (`local.CurMesh`) (`/Game/SmartAIMainFolder/Player/Preview/PDA_ClothesItem.Mesh` ClothesInfo))
  (`SceneComponent.K2_SetRelativeTransform` (`local.CurMesh`) (`/Game/SmartAIMainFolder/Player/Preview/PDA_ClothesItem.Position` ClothesInfo) false true)
  (`/Game/SmartAIMainFolder/Blueprints/Base/GI_Base.SetClothes` (`self.GIBase`) ClothesInfo))

(fn `UserConstructionScript`)