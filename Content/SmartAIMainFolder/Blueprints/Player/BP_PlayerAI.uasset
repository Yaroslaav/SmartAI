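; Player character for a top-down game that uses the Gameplay Ability System and can be possessed by either the player controller or its own AI controller.
; It stores both controllers and hands itself to the AI when the player controller unpossesses it.
; Gameplay messages for equipped slots spawn and attach items, granting abilities and passive effects, or remove effects by tag.
; Chosen-clothes restoration, health and patrol getters are stubs.
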(event `self.ReceivePossessed`
  (params (NewController :type "Controller Object Reference"))
  (bind _asbp_player_aicontroller (cast `/Game/SmartAIMainFolder/Blueprints/BP_PlayerAIController` NewController)
    (:`then`
      (set `self.AIController` _asbp_player_aicontroller)
      (`self.TryPossessAIController`))
    (:`CastFailed`
      (`parent.ReceivePossessed` NewController)
      (bind _asbp_top_down_controller (cast `/Game/TopDown/Blueprints/BP_TopDownController` NewController))
      (set `self.PlayerController` _asbp_top_down_controller))))

(event `self.ReceiveUnpossessed`
  (params (OldController :type "Controller Object Reference"))
  (cast `PlayerController` OldController)
  (`self.TryPossessAIController`))

(event `self.ReceiveBeginPlay`
  (`parent.ReceiveBeginPlay`)
  (bind _asgi_base (cast `/Game/SmartAIMainFolder/Blueprints/Base/GI_Base` (`GameplayStatics.GetGameInstance`)))
  (set `self.GIBase` _asgi_base)
  (`/Game/SmartAIMainFolder/GAS/I_ASCOwner.GrantAbilities` (`self.DefaultAbilities`))
  (`self.PutChosenClothes`)
  (`|ExecutionSequence`
    (:`then_0`
      (bind (_asynctaskproxy _actualchannel _payload) (`|AsyncAction_ListenForGameplayMessages` (struct :`TagName` "Message.Player.Inventory.EquippedSlots.AddItem") "/Game/SmartAIMainFolder/Player/Blueprints/Inventory/S_InventorySlot.S_InventorySlot")
        (:`then`
          (bind _asgi_base_2 (cast `/Game/SmartAIMainFolder/Blueprints/Base/GI_Base` (`GameplayStatics.GetGameInstance`)))
          (bind _output_get (set `self.GameInstance` _asgi_base_2))
          (`KismetSystemLibrary.PrintString` "call")
          (`/Game/SmartAIMainFolder/Blueprints/Base/GI_Base.OnPlayerSpawned` _output_get))
        (:`OnMessageReceived`
          (`self.EquipItem` (`.Item_4_A7E97CE746F81B3F8369048896645E3B` (break `/Game/SmartAIMainFolder/Player/Blueprints/Inventory/S_InventorySlot` _payload))))))
    (:`then_1`
      (bind (_asynctaskproxy_2 _actualchannel_2 _payload_2) (`|AsyncAction_ListenForGameplayMessages` (struct :`TagName` "Message.Player.Inventory.EquippedSlots.RemoveItem") "/Game/SmartAIMainFolder/Player/Blueprints/Inventory/S_InventorySlot.S_InventorySlot")
        (:`OnMessageReceived`
          (`AbilitySystemComponent.RemoveActiveEffectsWithTags` (`self.AbilitySystemComponent`) (`BlueprintGameplayTagLibrary.MakeGameplayTagContainerFromTag` (`/Game/SmartAIMainFolder/Player/Preview/PDA_Equipment.PassiveGameplayEffectTag` (`.Item_4_A7E97CE746F81B3F8369048896645E3B` (break `/Game/SmartAIMainFolder/Player/Blueprints/Inventory/S_InventorySlot` _payload_2))))))))))

(fn `ChangeCameraSpringArmLength`
  (params (Amount :type "Float (double-precision)"))
  (set `SpringArmComponent.TargetArmLength` (`KismetMathLibrary.FClamp` (+ (`SpringArmComponent.TargetArmLength` (`self.SpringArm`)) Amount) (`self.MinSpringArmLength`) (`self.MaxSpringArmLength`)) (`self.SpringArm`)))

(fn `Dash`
  (`AbilitySystemComponent.TryActivateAbilityByClass` (`self.AbilitySystemComponent`) "/Game/SmartAIMainFolder/GAS/Abilities/Player/GA_Dash.GA_Dash_C" true))

(fn `EquipItem`
  (params (Item :type "/Game/SmartAIMainFolder/Player/Preview/PDA_Equipment Object Reference"))
  (bind _returnvalue (`|SpawnActorFromClass` (`/Game/SmartAIMainFolder/Player/Preview/PDA_Equipment.ActorToSpawn` Item) (`/Game/SmartAIMainFolder/Player/Preview/PDA_Equipment.Position` Item) "Undefined" "MultiplyWithRoot" self null))
  (`self.K2_AttachToComponent` _returnvalue (`self.Mesh`) (`/Game/SmartAIMainFolder/Player/Preview/PDA_Equipment.Attach Socket` Item) "KeepRelative" "KeepRelative" "KeepRelative" true)
  (`self.GrandEquipmentAbilities` (`/Game/SmartAIMainFolder/Player/Preview/PDA_Equipment.Abilities` Item))
  (for _array_element (`/Game/SmartAIMainFolder/Player/Preview/PDA_Equipment.PassiveEffects` Item)
    (bind _returnvalue_2 (`AbilitySystemBlueprintLibrary.AssignTagSetByCallerMagnitude` (`AbilitySystemComponent.MakeOutgoingSpec` :`self` (`self.AbilitySystemComponent`) :`GameplayEffectClass` (break `/Game/SmartAIMainFolder/GAS/Effects/S_EffectToGrantInfo` _array_element)) (`.DataTag_8_C249B5934E10B844C74607B0ED16950C` (break `/Game/SmartAIMainFolder/GAS/Effects/S_EffectToGrantInfo` _array_element)) (`.Magnitude_5_5BFF74524360F49BFC1B38924FE93DFC` (break `/Game/SmartAIMainFolder/GAS/Effects/S_EffectToGrantInfo` _array_element))))
    (`AbilitySystemComponent.BP_ApplyGameplayEffectSpecToSelf` (`self.AbilitySystemComponent`) _returnvalue_2)))

(fn `GetAIController`
  (returns (AIController :type "/Game/SmartAIMainFolder/Blueprints/BP_PlayerAIController Object Reference"))
  (return (`self.AIController`)))

(fn `GetCharacterInfo`
  (returns (Info :type "/Game/SmartAIMainFolder/Blueprints/S_CharacterInfo Structure"))
  (return (`self.CharacterInfo`)))

(fn `GetCurrentHealth`
  (returns (NewParam :type "Float (double-precision)"))
  (return 0.0))

(fn `GetGrantedAbilitySpec`
  (params (Ability :type "GameplayAbility Class Reference"))
  (returns (SpecHandle :type "GameplayAbilitySpecHandle Structure") (Found :type Boolean))
  (bind (_value _returnvalue) (`BlueprintMapLibrary.Map_Find` (`self.GrantedAbilitiesSpec`) Ability))
  (return _value _returnvalue))

(fn `GetHeight`
  (returns (Height :type "Float (double-precision)"))
  (return (* (`CapsuleComponent.CapsuleHalfHeight` (`self.CapsuleComponent`)) 2.0)))

(fn `GetIdealRange`
  (returns (AttackRadius :type "Float (double-precision)") (DefendRadius :type "Float (double-precision)"))
  (return (`self.Attack Radius`) 0.0))

(fn `GetLastPointOfInterest`
  (returns (Point :type "Vector Structure"))
  (return (`self.LastpointOfInterest`)))

(fn `GetMaxHealth`
  (returns (NewParam :type "Float (double-precision)"))
  (return 0.0))

(fn `GetPatrolRoute`
  (returns (PatrolRoute :type "/Game/SmartAIMainFolder/Enemy/AI/BP_PatrolRoute Object Reference"))
  (return null))

(fn `GetPlayerController`
  (returns (OwnController :type "/Game/TopDown/Blueprints/BP_TopDownController Object Reference"))
  (return (`self.PlayerController`)))

(fn `GetSkeletalMesh`
  (returns (SkeletalMeshComponent :type "SkeletalMeshComponent Object Reference"))
  (return (`self.Mesh`)))

(fn `GetTarget`
  (returns (TargetActor :type "Actor Object Reference"))
  (return (`/Game/TopDown/Blueprints/BP_TopDownController.TargetActor` (`self.PlayerController`))))

(fn `GrandEquipmentAbilities`
  (params (Abilities :type "Array of /Game/SmartAIMainFolder/Weapons/S_EquippementAbilityInfo Structure"))
  (for _array_element Abilities
    (bind (_abilityforcharacter _abilityforcontroller) (break `/Game/SmartAIMainFolder/Weapons/S_EquippementAbilityInfo` _array_element))
    (`/Game/SmartAIMainFolder/GAS/I_ASCOwner.GrantAbility` _abilityforcharacter)
    (`/Game/SmartAIMainFolder/GAS/I_ASCOwner.GrantAbility` (`self.PlayerController`) _abilityforcontroller)
    (if (not true)
      (`GameplayMessageSubsystem.K2_BroadcastMessage` (subsystem `GameplayMessageSubsystem`) (struct :`TagName` "Message.Player.Inventory.EquippedSlots.AddItem") _array_element))))

(fn `GrantAbilities`
  (params (Abilities :type "Array of GameplayAbility Class Reference (by ref)"))
  (returns (Specs :type "Array of GameplayAbilitySpecHandle Structure"))
  (locals (GrantedSpecs :type "Array of GameplayAbilitySpecHandle Structure"))
  (for _array_element Abilities
    (bind _spec (`/Game/SmartAIMainFolder/GAS/I_ASCOwner.GrantAbility` _array_element))
    (`KismetArrayLibrary.Array_Add` (`local.GrantedSpecs`) _spec))
  (return (`local.GrantedSpecs`)))

(fn `GrantAbility`
  (params (Ability :type "GameplayAbility Class Reference"))
  (returns (Spec :type "GameplayAbilitySpecHandle Structure"))
  (if (`KismetSystemLibrary.IsValidClass` Ability)
    (bind _returnvalue (`AbilitySystemComponent.K2_GiveAbility` (`self.AbilitySystemComponent`) Ability 0 -1))
    (`BlueprintMapLibrary.Map_Add` (`self.GrantedAbilitiesSpec`) null _returnvalue)
    (return _returnvalue)
    (else
      (`KismetSystemLibrary.PrintString` "Abiltiy class to grant is invalid"))))

(fn `PossessAIController`
  (bind _playercontroller (`self.PlayerController`))
  (`Controller.UnPossess` _playercontroller)
  (`PlayerController.SetViewTargetWithBlend` _playercontroller self 0.0 "VTBlend_Linear" 0.0 false)
  (`self.TryPossessAIController`))

(fn `PutChosenClothes`)

(fn `PutClothes`
  (params (Info :type "/Game/SmartAIMainFolder/Player/Preview/PDA_Equipment Object Reference"))
  (locals (CoshesMesh :type "SkeletalMeshComponent Object Reference"))
  (switch `/Game/SmartAIMainFolder/Player/Preview/E_EquipmentItemType` (`/Game/SmartAIMainFolder/Player/Preview/PDA_Equipment.Type` Info)
    (:`NewEnumerator0`
      (set `local.CoshesMesh` (`self.Head`)))
    (:`NewEnumerator1`
      (set `local.CoshesMesh` (`self.Chest`)))
    (:`NewEnumerator3`
      (set `local.CoshesMesh` (`self.FootL`))))
  (`SkeletalMeshComponent.SetSkeletalMeshAsset` (`local.CoshesMesh`) (`/Game/SmartAIMainFolder/Player/Preview/PDA_Equipment.Mesh` Info))
  (`SceneComponent.K2_SetRelativeTransform` (`local.CoshesMesh`) (`/Game/SmartAIMainFolder/Player/Preview/PDA_Equipment.Position` Info) false true)
  (`/Game/SmartAIMainFolder/Blueprints/Base/GI_Base.SetClothes` (`self.GIBase`) Info)
  (for _array_element (`/Game/SmartAIMainFolder/Player/Preview/PDA_Equipment.Abilities` Info)
    (`/Game/SmartAIMainFolder/GAS/I_ASCOwner.GrantAbility` (break `/Game/SmartAIMainFolder/Weapons/S_EquippementAbilityInfo` _array_element))
    (`/Game/SmartAIMainFolder/GAS/I_ASCOwner.GrantAbility` (`self.PlayerController`) (`.AbilityForController_22_4B1527454D0C8E79E89E7E998A1145E1` (break `/Game/SmartAIMainFolder/Weapons/S_EquippementAbilityInfo` _array_element)))))

(fn `SetMovementSpeed`
  (params (Speed :type "/Game/SmartAIMainFolder/Enemy/Enums/E_MovementSpeed Enum" :default "NewEnumerator0"))
  (returns (SpeedValue :type "Float (double-precision)"))
  (bind _output_get (set `CharacterMovementComponent.MaxWalkSpeed` (select `/Game/SmartAIMainFolder/Enemy/Enums/E_MovementSpeed` Speed :`NewEnumerator1` 100.0 :`NewEnumerator2` 300.0 :`NewEnumerator3` 600.0 :!type "Float (single-precision)") (`self.CharacterMovement`)))
  (return _output_get))

(fn `SetPointOfInterest`
  (params (Point :type "Vector Structure"))
  (set `self.LastpointOfInterest` Point))

(fn `TryPossessAIController`
  (`/Engine/EditorBlueprintResources/StandardMacros.IsValid` (`self.GetController`)
    (:`Is Not Valid`
      (`Controller.Possess` (`self.AIController`) self)
      (`/Game/TopDown/Blueprints/BP_TopDownController.SetPLayerAIController` (`self.PlayerController`) (`self.AIController`)))))

(fn `UserConstructionScript`)