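; Main menu camera actor that jumps between preset viewpoints as the player moves through the menu and character customization.
; On BeginPlay it moves to the main menu position and binds to GSB_MainMenu game state events for menu open, customize tab open and clothes type select.
; Each event teleport-sets its location to the menu position, a full-body view, or a per-clothes-type position looked up in a map, without interpolation.
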(event `self.ReceiveBeginPlay`
  (`self.GoToMainMenuView`)
  (bind _asgsb_main_menu (cast `/Game/SmartAIMainFolder/Blueprints/Base/MainMenu/GSB_MainMenu` (`GameplayStatics.GetGameState`)))
  (bind _output_get (set `self.GameState` _asgsb_main_menu))
  (add `/Game/SmartAIMainFolder/Blueprints/Base/MainMenu/GSB_MainMenu.OnClothesTypeSelect` _output_get (delegate `OnClothesTypeSelect_Event`))
  (add `/Game/SmartAIMainFolder/Blueprints/Base/MainMenu/GSB_MainMenu.OnMainMenuOpen` (`self.GameState`) (delegate `OnMainMenuOpen_Event`))
  (add `/Game/SmartAIMainFolder/Blueprints/Base/MainMenu/GSB_MainMenu.OnCustomizeTabOpen` (`self.GameState`) (delegate `OnCustomizeTabOpen_Event`)))

(event `OnClothesTypeSelect_Event`
  (params (Type :type "/Game/SmartAIMainFolder/Player/Preview/E_EquipmentItemType Enum" :default "NewEnumerator0"))
  (`self.GoToClothesView` Type))

(event `OnMainMenuOpen_Event`
  (`self.GoToMainMenuView`))

(event `OnCustomizeTabOpen_Event`
  (`self.GoToCustomizeView`))

(fn `GoToClothesView`
  (params (ClothesType :type "/Game/SmartAIMainFolder/Player/Preview/E_EquipmentItemType Enum" :default "NewEnumerator0"))
  (`self.K2_SetActorLocation` (`BlueprintMapLibrary.Map_Find` (`self.CameraPositions`) ClothesType)))

(fn `GoToCustomizeView`
  (`self.K2_SetActorLocation` (`self.FullBodyView`)))

(fn `GoToMainMenuView`
  (`self.K2_SetActorLocation` self (`self.MainMenuPos`) false false))

(fn `UserConstructionScript`)