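; AI controller for BP_PlayerAI that turns player movement input into Behavior Tree states.
; On possess it runs the pawn's tree, starts Passive and seeds the Blackboard with attack radius and Ability System Component.
; Gameplay message listeners for FollowCursor and GoTo set movement type, point of interest and Walking, but only GoTo interrupts Attacking.
; Blackboard enum helpers gate state changes; the FollowCursor End listener has no handler.
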(event `self.ReceivePossess`
  (params (PossessedPawn :type "Pawn Object Reference"))
  (bind _asbp_player_ai (cast `/Game/SmartAIMainFolder/Blueprints/Player/BP_PlayerAI` PossessedPawn))
  (bind _output_get (set `self.As BP Player AI` _asbp_player_ai))
  (`self.RunBehaviorTree` (`/Game/SmartAIMainFolder/Blueprints/Player/BP_PlayerAI.BehaviorTree` _output_get))
  (`self.SetStateAsPassive`)
  (bind _attackradius (`/Game/SmartAIMainFolder/Blueprints/EnemyAi/BPI_Fighter.GetIdealRange` (`self.As BP Player AI`)))
  (`BlackboardComponent.SetValueAsFloat` (`self.Blackboard`) (`self.AttackRadiusKeyName`) _attackradius)
  (`BlackboardComponent.SetValueAsObject` (`self.Blackboard`) (`self.AbilitySystemComponentKeyName`) (`AbilitySystemBlueprintLibrary.GetAbilitySystemComponent` (`self.As BP Player AI`)))
  (`|ExecutionSequence`
    (:`then_0`
      (`|AsyncAction_ListenForGameplayMessages` (struct :`TagName` "Message.Player.Movement.FollowCursor.Start") "/Game/SmartAIMainFolder/Blueprints/S_Empty.S_Empty"
        (:`OnMessageReceived`
          (bind _state (`self.GetCurrentPlayerState`))
          (switch `/Game/SmartAIMainFolder/Enemy/Enums/E_AIStates` _state
            (:`NewEnumerator0`
              _)
            (:`NewEnumerator5`
              _))
          (`self.SetMovementTypeAs` "NewEnumerator0")
          (`self.SetStateAsWalking`))))
    (:`then_1`
      (`|AsyncAction_ListenForGameplayMessages` (struct :`TagName` "Message.Player.Movement.FollowCursor.End") "/Game/SmartAIMainFolder/Blueprints/S_Empty.S_Empty"))
    (:`then_2`
      (`|AsyncAction_ListenForGameplayMessages` (struct :`TagName` "Message.Player.Movement.GoTo.Start") "/Game/SmartAIMainFolder/Blueprints/S_Empty.S_Empty"
        (:`OnMessageReceived`
          (`KismetSystemLibrary.PrintString` "2")
          (bind _state_2 (`self.GetCurrentPlayerState`))
          (switch `/Game/SmartAIMainFolder/Enemy/Enums/E_AIStates` _state_2
            (:`NewEnumerator0`
              _)
            (:`NewEnumerator1`
              _)
            (:`NewEnumerator5`
              _))
          (`self.SetMovementTypeAs` "NewEnumerator1")
          (`self.SetStateAsWalking`))))))

(fn `GetCurrentPlayerState`
  (returns (State :type "/Game/SmartAIMainFolder/Enemy/Enums/E_AIStates Enum"))
  (return (cast `/Game/SmartAIMainFolder/Enemy/Enums/E_AIStates` (`BlackboardComponent.GetValueAsEnum` (`self.Blackboard`) (`self.StateKeyName`)))))

(fn `SetMovementTypeAs`
  (params (MovementType :type "/Game/SmartAIMainFolder/Enemy/Enums/E_MovementType Enum" :default "NewEnumerator0"))
  (`BlackboardComponent.SetValueAsEnum` (`self.Blackboard`) (`self.MovementTypeKeyName`) MovementType))

(fn `SetStateAs`
  (params (State :type "/Game/SmartAIMainFolder/Enemy/Enums/E_AIStates Enum" :default "NewEnumerator0"))
  (`BlackboardComponent.SetValueAsEnum` (`self.Blackboard`) (`self.StateKeyName`) State))

(fn `SetStateAsAttacking`
  (params (AttackTargetActor :type "Actor Object Reference"))
  (bind _state (`self.GetCurrentPlayerState`))
  (switch `/Game/SmartAIMainFolder/Enemy/Enums/E_AIStates` _state
    (:`NewEnumerator0`
      _)
    (:`NewEnumerator2`
      _)
    (:`NewEnumerator5`
      _))
  (`BlackboardComponent.SetValueAsObject` (`self.Blackboard`) (`self.AttackTargetKeyName`) AttackTargetActor)
  (`self.SetStateAs` "NewEnumerator1"))

(fn `SetStateAsPassive`
  (`self.SetStateAs` "NewEnumerator0"))

(fn `SetStateAsWalking`
  (bind _point (message `/Game/SmartAIMainFolder/Blueprints/I_Creature.GetLastPointOfInterest` (`self.As BP Player AI`)))
  (`BlackboardComponent.SetValueAsVector` (`self.Blackboard`) (`self.PointOfInterestKeyName`) _point)
  (`self.SetStateAs` "NewEnumerator5")
  (`self.GetCurrentPlayerState`))

(fn `UserConstructionScript`)