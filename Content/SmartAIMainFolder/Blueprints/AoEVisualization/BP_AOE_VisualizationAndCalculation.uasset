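; Area-of-effect telegraph actor that shows a decal and warns pawns inside it of an incoming hit.
; BeginPlay scales the trigger, NavMeshDestroyer and decal from a shared Scale, applies the decal material and optionally attaches to the instigator.
; Tick sends a WillGetHit.AoE gameplay event to overlapping pawns lacking that tag, then adds it as a non-replicated loose tag, which suppresses repeat events.
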(event `self.ReceiveBeginPlay`
  (bind _asgmb_game (cast `/Game/SmartAIMainFolder/Blueprints/Base/Game/GMB_Game` (`GameplayStatics.GetGameMode`)))
  (bind _output_get (set `self.As GMB Game` _asgmb_game))
  (`/Game/SmartAIMainFolder/Blueprints/Base/Game/GMB_Game.GetUndergroundOffset` _output_get)
  (`self.SetShapeSize`)
  (`DecalComponent.SetDecalMaterial` (`self.Decal`) (`self. Decal Material`))
  (if (`self.AttachToOwner`)
    (`self.K2_AttachToActor` (`self.Instigator`) "None" "KeepWorld" "KeepRelative" "KeepRelative")))

(event `self.ReceiveTick`
  (params (DeltaSeconds :type "Float (single-precision)"))
  (for _array_element (`PrimitiveComponent.GetOverlappingActors` (`self.Trigger`) "/Script/Engine.Pawn")
    (bind _returnvalue (message `GameplayTagAssetInterface.HasAnyMatchingGameplayTags` (`AbilitySystemBlueprintLibrary.GetAbilitySystemComponent` _array_element) (`BlueprintGameplayTagLibrary.MakeLiteralGameplayTagContainer` (struct :`GameplayTags` (struct :`(TagName` "Entity.Combat.WillGetHit.AoE"))))))
    (if (not _returnvalue)
      (`AbilitySystemBlueprintLibrary.SendGameplayEventToActor` _array_element (struct :`TagName` "Entity.Combat.WillGetHit.AoE") (make `GameplayEventData` (struct :`TagName` "Entity.Combat.WillGetHit.AoE") self))
      (`AbilitySystemBlueprintLibrary.AddLooseGameplayTags` _array_element (`BlueprintGameplayTagLibrary.MakeLiteralGameplayTagContainer` (struct :`GameplayTags` (struct :`(TagName` "Entity.Combat.WillGetHit.AoE"))))))))

(fn `SetShapeSize`
  (bind _returnvalue (/ (`self.Scale`) 50.0))
  (`SceneComponent.SetWorldScale3D` (`self.Trigger`) _returnvalue)
  (`SceneComponent.SetWorldScale3D` (`self.NavMeshDestroyer`) _returnvalue)
  (`SceneComponent.SetWorldScale3D` (`self.Decal`) (`self.Scale`)))

(fn `UserConstructionScript`)