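; Blueprint math function library for the SmartAI system with one helper, ClampLocationInRadius, which constrains a location around a center point.
; It flattens the offset between the two points to the XY plane, clamps its length between a small fixed minimum and Radius, and applies it from Center.
; The returned point therefore takes Center's height, discarding the input location's Z.
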(fn `ClampLocationInRadius`
  (params (Center :type "Vector Structure") (Location :type "Vector Structure") (Radius :type "Float (double-precision)"))
  (returns (Result :type "Vector Structure"))
  (return (+ (`local.Center`) (* (`KismetMathLibrary.ClampVectorSize` (- (`KismetMathLibrary.MakeVector` (.x Center) (.y Center) (.z Location)) (`local.Location`)) 10.0 (`local.Radius`)) -1.0))))