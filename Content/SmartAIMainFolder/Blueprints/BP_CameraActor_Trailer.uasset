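; Camera actor, named for trailer use, that flies its camera component along a spline.
; After a half-second delay from BeginPlay, Tick advances the distance along the spline by Speed scaled by delta time.
; Each frame the camera's relative location and rotation are set from the spline's local-space transform at that distance, with no end or loop check.
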(event `self.ReceiveBeginPlay`
  (`KismetSystemLibrary.Delay` 0.5)
  (set `self.CanGo` true))

(event `self.ReceiveTick`
  (params (DeltaSeconds :type "Float (single-precision)"))
  (bind (_returnvalue_location _returnvalue_rotation) (`KismetMathLibrary.BreakTransform` (`SplineComponent.GetTransformAtDistanceAlongSpline` (`self.Spline`) (`self.DistanceAlongSpline`) "Local" false)))
  (if (`self.CanGo`)
    (set `self.DistanceAlongSpline` (+ (* DeltaSeconds (`self.Speed`)) (`self.DistanceAlongSpline`)))
    (`SceneComponent.K2_SetRelativeTransform` (`self.CameraComponent`) (`KismetMathLibrary.MakeTransform` _returnvalue_location _returnvalue_rotation) false false)))

(fn `UserConstructionScript`)