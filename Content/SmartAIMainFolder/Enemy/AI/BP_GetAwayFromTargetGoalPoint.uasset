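; BP_GetAwayFromTargetGoalPoint is a helper actor in the enemy AI folder that marks a goal point for a Querier to get away from its Target.
; CalcAndSetPosition projects a fixed distance beyond the Querier along the Target-to-Querier look-at direction, keeping the Querier's height.
; It runs on BeginPlay and then on a short looping timer, so the point follows both actors' movement without Tick.
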(event `self.ReceiveBeginPlay`
  (`self.CalcAndSetPosition`)
  (`KismetSystemLibrary.K2_SetTimerDelegate` (delegate `ChangePosition`) 0.1 true))

(event `ChangePosition`
  (`self.CalcAndSetPosition`))

(fn `CalcAndSetPosition`
  (bind _returnvalue (`self.K2_GetActorLocation` (`self.Querier`)))
  (`self.K2_SetActorLocation` (`KismetMathLibrary.MakeVector` (.x (+ (* (`KismetMathLibrary.GetForwardVector` (`KismetMathLibrary.FindLookAtRotation` (`self.K2_GetActorLocation` (`self.Target`)) _returnvalue)) 1000.0) (`self.K2_GetActorLocation` (`self.Querier`)))) (.y (+ (* (`KismetMathLibrary.GetForwardVector` (`KismetMathLibrary.FindLookAtRotation` (`self.K2_GetActorLocation` (`self.Target`)) _returnvalue)) 1000.0) (`self.K2_GetActorLocation` (`self.Querier`)))) (.z _returnvalue))))

(fn `UserConstructionScript`)