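; Gameplay ability for a one-handed dagger auto attack in a top-down game, currently an unfinished prototype that only moves toward the target.
; On activation it caches the avatar's top-down controller, gets the target from the avatar and calls SimpleMoveToActor.
; The attack-range check, overlap wait and movement-end binding are unwired, and Attack is empty.
; Ability end only prints whether the controller is valid.
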(event `self.K2_ActivateAbility`
  (bind _ascharacter (cast `Character` (`self.GetAvatarActorFromActorInfo`)))
  (bind _asbp_top_down_controller (cast `/Game/TopDown/Blueprints/BP_TopDownController` (`Pawn.GetController` _ascharacter)))
  (bind _output_get (set `self.PlayerController` _asbp_top_down_controller))
  (bind _targetactor (message `/Game/SmartAIMainFolder/Blueprints/EnemyAi/BPI_Fighter.GetTarget` (`self.GetAvatarActorFromActorInfo`)))
  (bind _output_get_2 (set `self.AttackTarget` _targetactor))
  (`AIBlueprintHelperLibrary.SimpleMoveToActor` _output_get _output_get_2))

(event `OnMovementEnd_Event`
  (params (Cancelled :type Boolean)))

(event `self.K2_OnEndAbility`
  (params (bWasCancelled :type Boolean))
  (`KismetSystemLibrary.PrintString` (`KismetStringLibrary.Conv_BoolToString` (`KismetSystemLibrary.IsValid` (`self.PlayerController`)))))

(fn `Attack`)