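; GA_MoveToLocation is a Gameplay Ability that moves the player to the top-down controller's cached click destination.
; On activation it stops current movement, spawns an end-trigger actor sized by IdealRange at the destination, starts SimpleMoveToLocation and spawns a cursor effect.
; The controller's movement-end event ends or cancels the ability.
; Ending destroys the trigger and stops movement if cancelled.
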(event `self.K2_ActivateAbility`
  (bind _cacheddestination (`/Game/TopDown/Blueprints/BP_TopDownController.CachedDestination` (`self.Conroller`)))
  (bind _returnvalue (`self.K2_CommitAbility`))
  (if _returnvalue
    (bind _asbp_player (cast `/Game/SmartAIMainFolder/Blueprints/Player/BP_Player` (`self.GetAvatarActorFromActorInfo`)))
    (bind _output_get (set `self.BPPlayer` _asbp_player))
    (bind _asbp_top_down_controller (cast `/Game/TopDown/Blueprints/BP_TopDownController` (`Pawn.GetController` _output_get)))
    (bind _output_get_2 (set `self.Conroller` _asbp_top_down_controller))
    (`Controller.StopMovement` _output_get_2)
    (bind _returnvalue_2 (`|SpawnActorFromClass` "/Game/SmartAIMainFolder/Blueprints/Player/Movement/BP_CharacterSimpleMovementEndTrigger.BP_CharacterSimpleMovementEndTrigger_C" (`KismetMathLibrary.MakeTransform` _cacheddestination) "AlwaysSpawn" "MultiplyWithRoot" null (`self.IdealRange`) (`self.BPPlayer`) null))
    (set `self.EndMovementTrigger` _returnvalue_2)
    (add `/Game/TopDown/Blueprints/BP_TopDownController.OnMovementEnd` (`self.Conroller`) (delegate `OnMovementEnd_Event`))
    (`AIBlueprintHelperLibrary.SimpleMoveToLocation` _output_get_2 _cacheddestination)
    (`NiagaraFunctionLibrary.SpawnSystemAtLocation` "/Game/Cursor/FX_Cursor.FX_Cursor" _cacheddestination)
    (else
      (`self.K2_CancelAbility`))))

(event `OnMovementEnd_Event`
  (params (Cancelled :type Boolean))
  (if Cancelled
    (`self.K2_CancelAbility`)
    (else
      (`self.K2_EndAbility`))))

(event `self.K2_OnEndAbility`
  (params (bWasCancelled :type Boolean))
  (bind _endmovementtrigger (`self.EndMovementTrigger`))
  (bind _conroller (`self.Conroller`))
  (`KismetSystemLibrary.PrintString` (`KismetStringLibrary.Concat_StrStr` "End movement: " (`KismetStringLibrary.Conv_BoolToString` bWasCancelled)))
  (`/Engine/EditorBlueprintResources/StandardMacros.IsValid` _endmovementtrigger
    (:`Is Valid`
      (`Actor.K2_DestroyActor` _endmovementtrigger)
      (if bWasCancelled
        (`/Engine/EditorBlueprintResources/StandardMacros.IsValid` _conroller
          (:`Is Valid`
            (`Controller.StopMovement` _conroller)))))))