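; Gameplay Ability for an enemy AI melee attack that plays an outward sword slash montage and damages the target it hits.
; After committing, it runs the montage while listening for Event.HitTarget, ending on completion and cancelling on interruption.
; Each valid hit applies GE_ApplyDamage from instigator to target, passing the Damage variable as a Calculation.Damage SetByCaller magnitude.
; CalculateDamage is an unused stub returning zero.
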(event `self.K2_ActivateAbility`
  (bind _returnvalue (`self.K2_CommitAbility`))
  (if _returnvalue
    (`AbilityTask_PlayMontageAndWait.CreatePlayMontageAndWaitProxy` "None" "/Game/SmartAIMainFolder/Animations/Montages/StableSwordOutwardSlash_UE_Montage.StableSwordOutwardSlash_UE_Montage"
      (:`then`
        (bind _asynctaskproxy (`AbilityTask_WaitGameplayEvent.WaitGameplayEvent` (struct :`TagName` "Event.HitTarget") null)
          (:`then`
            (add `AbilityTask_WaitGameplayEvent.EventReceived` _asynctaskproxy (delegate `EventReceived_Event`)))))
      (:`OnCompleted`
        (`self.K2_EndAbility`))
      (:`OnInterrupted`
        (`self.K2_CancelAbility` :!label _label))
      (:`OnCancelled`
        (goto _label)))
    (else
      (`self.K2_CancelAbility`))))

(event `EventReceived_Event`
  (params (Payload :type "GameplayEventData Structure"))
  (bind (_eventtag _instigator _target) (break `GameplayEventData` Payload))
  (if (and (`KismetSystemLibrary.IsValid` _instigator) (`KismetSystemLibrary.IsValid` _target))
    (bind _returnvalue (`AbilitySystemBlueprintLibrary.AssignTagSetByCallerMagnitude` (`AbilitySystemComponent.MakeOutgoingSpec` :`self` (`AbilitySystemBlueprintLibrary.GetAbilitySystemComponent` _instigator) :`GameplayEffectClass` "/Game/SmartAIMainFolder/GAS/Effects/Damage/GE_ApplyDamage.GE_ApplyDamage_C") (struct :`TagName` "Calculation.Damage") (`self.Damage`)))
    (`AbilitySystemComponent.BP_ApplyGameplayEffectSpecToTarget` (`AbilitySystemBlueprintLibrary.GetAbilitySystemComponent` _instigator) _returnvalue (`AbilitySystemBlueprintLibrary.GetAbilitySystemComponent` _target))
    (else
      (`self.K2_CancelAbility`))))

(event `self.K2_OnEndAbility`
  (params (bWasCancelled :type Boolean)))

(fn `CalculateDamage`
  (returns (Damage :type "Float (double-precision)"))
  (return 0.0))