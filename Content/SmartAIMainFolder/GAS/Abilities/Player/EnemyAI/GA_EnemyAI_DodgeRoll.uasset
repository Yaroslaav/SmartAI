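; GA_EnemyAI_DodgeRoll is an event-triggered gameplay ability that dashes the avatar in a dodge.
; It takes the hit location from the event's target data, faces a direction toward it, and projects DodgeMaxDistance along it.
; After committing, a short root-motion move-to force drives the movement in walking mode, then ends the ability.
; A failed commit cancels, and ability end also commits cooldown.
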(event `self.K2_ActivateAbilityFromEvent`
  (params (EventData :type "GameplayEventData Structure (by ref)"))
  (bind _returnvalue (`self.K2_CommitAbility`))
  (if _returnvalue
    (`AbilityTask_ApplyRootMotionMoveToForce.ApplyRootMotionMoveToForce` "None" (+ (* (`KismetMathLibrary.GetForwardVector` (`KismetMathLibrary.FindLookAtRotation` (`Actor.K2_GetActorLocation` (`self.GetAvatarActorFromActorInfo`)) (`.Location` (`GameplayStatics.BreakHitResult` (`AbilitySystemBlueprintLibrary.GetHitResultFromTargetData` (`.TargetData` (break `GameplayEventData` EventData))))))) (`self.DodgeMaxDistance`)) (`Actor.K2_GetActorLocation` (`self.GetAvatarActorFromActorInfo`))) 0.2 true "MOVE_Walking" false null "SetVelocity"
      (:`OnTimedOut`
        _)
      (:`OnTimedOutAndDestinationReached`
        _))
    (`self.K2_EndAbility`)
    (else
      (`self.K2_CancelAbility`))))

(event `self.K2_OnEndAbility`
  (params (bWasCancelled :type Boolean))
  (`self.K2_CommitAbilityCooldown` true))