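; Gameplay ability for a player fireball that charges while input is held and fires on release.
; On activation it spawns a BP_Fireball attached above the owner's origin and passes it max size and full-charge time.
; Releasing after a minimum hold shoots it along the owner's forward vector at a level scaled from hold time, capped at MaxLevel.
; Shorter holds cancel the ability, which destroys the fireball.
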(event `self.K2_ActivateAbility`
  (bind _returnvalue (`self.GetOwningActorFromActorInfo`))
  (set `self.TimeToLevelUp` (/ (`self.TimeToFullCharge`) (`self.MaxLevel`)))
  (bind (_asynctaskproxy _timeheld) (`AbilityTask_WaitInputRelease.WaitInputRelease` false)
    (:`then`
      (bind _returnvalue_2 (`|SpawnActorFromClass` "/Game/SmartAIMainFolder/GAS/Abilities/Player/FireBall/BP_Fireball.BP_Fireball_C" (`KismetMathLibrary.MakeTransform` (+ (`Actor.K2_GetActorLocation` _returnvalue) (0.0 0.0 50.0)) (`KismetMathLibrary.Conv_VectorToRotator` (`Actor.GetActorForwardVector` _returnvalue))) "AlwaysSpawn" "MultiplyWithRoot" _returnvalue null))
      (`Actor.K2_AttachToActor` _returnvalue_2 (`self.GetOwningActorFromActorInfo`) "None" "KeepWorld" "KeepRelative" "KeepRelative" true)
      (bind _output_get (set `self.As BP Fireball` _returnvalue_2))
      (`/Game/SmartAIMainFolder/GAS/Abilities/Player/FireBall/BP_Fireball.SetInfo` _output_get (`self.MaxSize`) (`self.TimeToFullCharge`)))
    (:`OnRelease`
      (if (< (`self.MinThreshold`) _timeheld)
        (`/Game/SmartAIMainFolder/GAS/Abilities/Player/FireBall/BP_Fireball.Shoot` (`self.As BP Fireball`) (`KismetMathLibrary.FTrunc` (`KismetMathLibrary.FClamp` (/ _timeheld (`self.TimeToLevelUp`)) 0.0 (`self.MaxLevel`))) (`Actor.GetActorForwardVector` (`self.GetOwningActorFromActorInfo`)))
        (`self.K2_EndAbility`)
        (else
          (`self.K2_CancelAbility`))))))

(event `self.K2_OnEndAbility`
  (params (bWasCancelled :type Boolean))
  (if bWasCancelled
    (`Actor.K2_DestroyActor` (`self.As BP Fireball`))))