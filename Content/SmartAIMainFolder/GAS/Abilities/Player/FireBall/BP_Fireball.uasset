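; Chargeable fireball projectile for the player's GAS ability, which grows while held and deals damage once launched.
; SetInfo derives a growth rate, and Tick scales the sphere until the charge time runs out or it is shot.
; Shoot detaches it, activates projectile movement along the given direction and starts the lifetime countdown.
; Once shot, overlapping a non-owner applies GE_FireballDamage at the passed level and destroys it.
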(event `self.ReceiveBeginPlay`
  (`ActorComponent.Deactivate` (`self.ProjectileMovement`))
  (add `self.OnShoot` (delegate `OnShoot_Event`)))

(event `OnShoot_Event`
  (`KismetSystemLibrary.Delay` (`self.LifeTime`))
  (`self.K2_DestroyActor`))

(event `self.ReceiveTick`
  (params (DeltaSeconds :type "Float (single-precision)"))
  (if (and (> (`self.TimeToFullCharge`) 0.0) (not (`self.Charged`)))
    (`self.Rise` DeltaSeconds)))

(event `self.Sphere.OnComponentBeginOverlap`
  (params (OverlappedComponent :type "PrimitiveComponent Object Reference") (OtherActor :type "Actor Object Reference") (OtherComp :type "PrimitiveComponent Object Reference") (OtherBodyIndex :type Integer) (bFromSweep :type Boolean) (SweepResult :type "HitResult Structure (by ref)"))
  (bind _returnvalue (`self.GetOwner`))
  (if (`self.Charged`)
    (if (!= OtherActor _returnvalue)
      (`AbilitySystemComponent.BP_ApplyGameplayEffectToTarget` :`self` (`AbilitySystemBlueprintLibrary.GetAbilitySystemComponent` _returnvalue) :`GameplayEffectClass` "/Game/SmartAIMainFolder/GAS/Effects/Damage/GE_FireballDamage.GE_FireballDamage_C" :`Target` (`AbilitySystemBlueprintLibrary.GetAbilitySystemComponent` OtherActor) :`Level` (`KismetMathLibrary.Conv_IntToDouble` (`self.Level`)))
      (`self.K2_DestroyActor`))))

(fn `Rise`
  (params (DelatSeconds :type "Float (double-precision)"))
  (locals (CurrentRise :type "Float (double-precision)"))
  (bind _currentrise (`local.CurrentRise`))
  (set `self.TimeToFullCharge` (- (`self.TimeToFullCharge`) DelatSeconds))
  (set `local.CurrentRise` (* (`self.SizePerSecond`) DelatSeconds))
  (`SceneComponent.SetWorldScale3D` (`self.Sphere`) (+ (`SceneComponent.K2_GetComponentScale` (`self.Sphere`)) (`KismetMathLibrary.MakeVector` _currentrise _currentrise _currentrise))))

(fn `SetInfo`
  (params (MaxSize :type "Float (double-precision)") (TimeToFullCharge :type "Float (double-precision)"))
  (bind _returnvalue_x (`KismetMathLibrary.BreakVector` (`SceneComponent.K2_GetComponentScale` (`self.Sphere`))))
  (bind _output_get (set `self.MaxSize` MaxSize))
  (bind _output_get_2 (set `self.TimeToFullCharge` TimeToFullCharge))
  (set `self.SizePerSecond` (/ (- _output_get _returnvalue_x) _output_get_2)))

(fn `Shoot`
  (params (Level :type Integer) (Direction :type "Vector Structure"))
  (bind _projectilemovement (`self.ProjectileMovement`))
  (bind _speed (`self.Speed`))
  (`self.K2_DetachFromActor` "KeepWorld")
  (set `self.Level` Level)
  (set `self.Charged` true)
  (`ActorComponent.Activate` _projectilemovement false)
  (set `MovementComponent.Velocity` (* Direction (`KismetMathLibrary.MakeVector` _speed _speed _speed)) _projectilemovement)
  (`KismetSystemLibrary.PrintString` (`KismetStringLibrary.Conv_VectorToString` (`MovementComponent.Velocity` _projectilemovement)))
  (`self.OnShoot`))

(fn `UserConstructionScript`)