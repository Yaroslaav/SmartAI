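; Player gameplay ability that sends the BP_PlayerAI avatar to its last point of interest through its AI controller.
; On activation it stops current movement, starts a non-pathfinding AI MoveTo and spawns a cursor effect at the destination.
; The move result ends or cancels the ability.
; On cancel, a Walking state re-issues the move to the latest point, while other states switch movement type, then the async task is cleaned up.
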(event `self.K2_ActivateAbility`
  (bind _returnvalue (`self.K2_CommitAbility`))
  (if _returnvalue
    (bind _asbp_player_ai (cast `/Game/SmartAIMainFolder/Blueprints/Player/BP_PlayerAI` (`self.GetAvatarActorFromActorInfo`)))
    (bind _output_get (set `self.BPPlayer` _asbp_player_ai))
    (bind _aicontroller (`/Game/SmartAIMainFolder/Blueprints/Player/BP_PlayerAI.GetAIController` _output_get))
    (bind _output_get_2 (set `self.Conroller` _aicontroller))
    (`Controller.StopMovement` _output_get_2)
    (bind _point (`/Game/SmartAIMainFolder/Blueprints/I_Creature.GetLastPointOfInterest` (`self.BPPlayer`)))
    (bind _output_get_3 (set `self.Dest` _point))
    (bind _asynctaskproxy (`AITask_MoveTo.AIMoveTo` (`self.Conroller`) _output_get_3 null 20.0 "Enable" "Default" false false)
      (:`then`
        (set `self.Async Task` _asynctaskproxy)
        (`NiagaraFunctionLibrary.SpawnSystemAtLocation` "/Game/Cursor/FX_Cursor.FX_Cursor" _output_get_3)
        (switch `EPathFollowingStatus` (`AIController.GetMoveStatus` (`self.Conroller`))
          (:`Idle`
            (`KismetSystemLibrary.PrintString` "Idl;e")
            (`self.K2_EndAbility`))))
      (:`OnRequestFailed`
        (`self.K2_CancelAbility`))
      (:`OnMoveFinished`
        (`self.K2_EndAbility`)))
    (else
      (`self.K2_CancelAbility`))))

(event `self.K2_OnEndAbility`
  (params (bWasCancelled :type Boolean))
  (bind _conroller (`self.Conroller`))
  (bind _async_task (`self.Async Task`))
  (if bWasCancelled
    (bind _point (`/Game/SmartAIMainFolder/Blueprints/I_Creature.GetLastPointOfInterest` (`self.BPPlayer`)))
    (`/Engine/EditorBlueprintResources/StandardMacros.IsValid` _conroller
      (:`Is Valid`
        (bind _state (`/Game/SmartAIMainFolder/Blueprints/BP_PlayerAIController.GetCurrentPlayerState` _conroller))
        (switch `/Game/SmartAIMainFolder/Enemy/Enums/E_AIStates` _state
          (:`NewEnumerator0`
            (`/Game/SmartAIMainFolder/Blueprints/BP_PlayerAIController.SetMovementTypeAs` _conroller "NewEnumerator2" :!label _label))
          (:`NewEnumerator1`
            (goto _label))
          (:`NewEnumerator2`
            (goto _label))
          (:`NewEnumerator5`
            (`AIController.MoveToLocation` _conroller _point 20.0 true false false true null true))))))
  (`/Engine/EditorBlueprintResources/StandardMacros.IsValid` _async_task
    (:`Is Valid`
      (`GameplayTask.EndTask` _async_task))))