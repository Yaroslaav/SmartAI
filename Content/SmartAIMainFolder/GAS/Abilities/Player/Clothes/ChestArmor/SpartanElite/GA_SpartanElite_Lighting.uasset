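; Player gameplay ability for the Spartan Elite chest armor that surrounds the character with a damaging lightning aura for a set duration.
; After committing cost, it attaches a Niagara effect scaled to the radius and starts end and looping damage timers.
; Each damage tick sphere-overlaps enemy AI and applies a damage GameplayEffect using SetByCaller magnitude.
; Cooldown is committed only when the aura expires and the effect is destroyed.
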(event `self.K2_ActivateAbility`
  (bind _returnvalue (`self.K2_CommitAbilityCost` true))
  (if _returnvalue
    (bind _ascharacter (cast `Character` (`self.GetAvatarActorFromActorInfo`)))
    (bind _output_get (set `self.As Character` _ascharacter))
    (bind _returnvalue_2 (`NiagaraFunctionLibrary.SpawnSystemAttached` "/Game/SmartAIMainFolder/Niagara/NS_Lighting.NS_Lighting" (`Character.CapsuleComponent` _output_get) "None" (0.0 0.0 0.0) (struct) "KeepRelativeOffset"))
    (bind _output_get_2 (set `self.GCN` _returnvalue_2))
    (`SceneComponent.SetWorldScale3D` _output_get_2 (`KismetMathLibrary.Conv_DoubleToVector` (/ (`self.AbilityRadius`) 100.0)))
    (`KismetSystemLibrary.K2_SetTimerDelegate` (delegate `End`) (`self.Duration`))
    (`KismetSystemLibrary.K2_SetTimerDelegate` (delegate `Damage`) 0.1 true)
    (else
      (`self.K2_CancelAbility`))))

(event `Damage`
  (bind _outactors (`KismetSystemLibrary.SphereOverlapActors` (`Actor.K2_GetActorLocation` (`self.As Character`)) (`self.AbilityRadius`) (`|MakeArray` "ObjectTypeQuery3" :!type "EObjectTypeQuery Enum") "/Game/SmartAIMainFolder/Blueprints/EnemyAi/BP_EnemyAI_Base.BP_EnemyAI_Base_C" (`|MakeArray` (`self.As Character`) :!type "Actor Object Reference")))
  (for _array_element _outactors
    (bind _asbp_enemy_ai_base (cast `/Game/SmartAIMainFolder/Blueprints/EnemyAi/BP_EnemyAI_Base` _array_element))
    (bind _returnvalue (`AbilitySystemBlueprintLibrary.AssignTagSetByCallerMagnitude` (`AbilitySystemComponent.MakeOutgoingSpec` :`self` (`AbilitySystemBlueprintLibrary.GetAbilitySystemComponent` (`self.As Character`)) :`GameplayEffectClass` "/Game/SmartAIMainFolder/GAS/Abilities/Player/Clothes/ChestArmor/SpartanElite/GE_SpartanElite_LightingDamage.GE_SpartanElite_LightingDamage_C") (struct :`TagName` "Calculation.Damage") (`self.HitDamage`)))
    (`AbilitySystemComponent.BP_ApplyGameplayEffectSpecToTarget` (`AbilitySystemBlueprintLibrary.GetAbilitySystemComponent` (`self.As Character`)) _returnvalue (`AbilitySystemBlueprintLibrary.GetAbilitySystemComponent` _asbp_enemy_ai_base))))

(event `End`
  (`ActorComponent.K2_DestroyComponent` (`self.GCN`))
  (`self.K2_CommitAbilityCooldown` true)
  (`self.K2_EndAbility`))