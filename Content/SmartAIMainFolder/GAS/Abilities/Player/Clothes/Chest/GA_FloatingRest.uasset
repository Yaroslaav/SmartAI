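; Player chest-clothing gameplay ability that puts the owner into a floating rest, backed by the GE_FloatingRest effect.
; Activation applies the effect, plays a floating montage and waits for the effect's removal or an invalid handle to end the ability.
; Ending stops the montage, commits the cooldown and removes the effect, with the EffectWasCancelled flag intended to guard against repeated teardown.
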(event `self.K2_ActivateAbility`
  (bind _returnvalue (`self.BP_ApplyGameplayEffectToOwner` "/Game/SmartAIMainFolder/GAS/Abilities/Player/Clothes/Chest/Effects/GE_FloatingRest.GE_FloatingRest_C"))
  (bind _output_get (set `self.ActiveEffect` _returnvalue))
  (`AbilityTask_WaitGameplayEffectRemoved.WaitForGameplayEffectRemoved` _output_get
    (:`then`
      (`AbilityTask_PlayMontageAndWait.CreatePlayMontageAndWaitProxy` "None" "/Game/SmartAIMainFolder/Animations/Montages/FloatingManny_Montage.FloatingManny_Montage"))
    (:`OnRemoved`
      (if (not (`self.EffectWasCancelled`)) :!label _label
        (`self.K2_EndAbility`)
        (set `self.EffectWasCancelled` true)))
    (:`InvalidHandle`
      (goto _label))))

(event `self.K2_OnEndAbility`
  (params (bWasCancelled :type Boolean))
  (`self.MontageStop` -1.0)
  (`self.K2_CommitAbilityCooldown` false)
  (if (not (`self.EffectWasCancelled`))
    (set `self.EffectWasCancelled` true)
    (`self.BP_RemoveGameplayEffectFromOwnerWithHandle` (`self.ActiveEffect`))))