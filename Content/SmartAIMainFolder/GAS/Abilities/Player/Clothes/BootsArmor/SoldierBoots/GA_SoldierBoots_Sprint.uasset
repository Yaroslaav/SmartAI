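; Soldier Boots sprint ability that grants the player a timed speed boost.
; On commit of cost, it applies GE_SoldierBoots_SpeedBoost with SetByCaller duration and a magnitude scaled from base speed, then broadcasts the buff info on a gameplay message channel.
; It then commits cooldown and starts a looping timer that spawns a Niagara effect at the character's location.
; The ability ends when the effect is removed.
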(event `self.K2_ActivateAbility`
  (bind _returnvalue (`self.K2_CommitAbilityCost` true))
  (if _returnvalue
    (bind _returnvalue_2 (`AbilitySystemBlueprintLibrary.AssignTagSetByCallerMagnitude` (`self.MakeOutgoingGameplayEffectSpec` "/Game/SmartAIMainFolder/GAS/Abilities/Player/Clothes/BootsArmor/SoldierBoots/GE_SoldierBoots_SpeedBoost.GE_SoldierBoots_SpeedBoost_C") (struct :`TagName` "Effect.Info.Duration") (`self.Duration`)))
    (bind _speed (message `/Game/SmartAIMainFolder/Blueprints/EnemyAi/BPI_Fighter.GetBaseSpeed` (`self.GetAvatarActorFromActorInfo`)))
    (bind _returnvalue_3 (`AbilitySystemBlueprintLibrary.AssignTagSetByCallerMagnitude` _returnvalue_2 (struct :`TagName` "Effect.Info.Magnitude") (* _speed (`self.Magnitude`))))
    (bind _returnvalue_4 (`self.K2_ApplyGameplayEffectSpecToOwner` _returnvalue_3))
    (set `self.SpeedBoostEffect` _returnvalue_4)
    (`GameplayMessageSubsystem.K2_BroadcastMessage` (subsystem `GameplayMessageSubsystem`) (struct :`TagName` "Effect.Active.Buff.SpeedBoost") (make `/Game/SmartAIMainFolder/Blueprints/S_PlayerActiveGameplayEffectInfo` (`self.GetAvatarActorFromActorInfo`) (`self.SpeedBoostEffect`) (`self.Magnitude`) (`self.Duration`) (`self.SpeedBoostIcon`)))
    (`AbilityTask_WaitGameplayEffectRemoved.WaitForGameplayEffectRemoved` (`self.SpeedBoostEffect`)
      (:`then`
        (bind _ascharacter (cast `Character` (`self.GetAvatarActorFromActorInfo`)))
        (set `self.Character` _ascharacter)
        (`KismetSystemLibrary.K2_SetTimerDelegate` (delegate `SpawnCue`) 0.1 true)
        (`self.K2_CommitAbilityCooldown` true))
      (:`OnRemoved`
        (`self.K2_EndAbility`))
      (:`InvalidHandle`
        (`self.K2_CancelAbility`)))))

(event `SpawnCue`
  (`NiagaraFunctionLibrary.SpawnSystemAtLocation` "/Game/sA_PickupSet_1/Fx/NiagaraSystems/NS_Healing_1.NS_Healing_1" (`Actor.K2_GetActorLocation` (`self.Character`)) (struct) (0.7 0.7 0.7)))