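; Player dash ability that moves the character toward the cursor, clamped to a max radius, and deals area damage.
; It stops AI movement, then runs a root-motion move with an optional montage.
; When the move finishes, it ends the ability, then spawns a hit sphere, placed or attached per DamageType, applying the Bloodletter damage effect through GAS.
; On end, it restores Walking or sets Passive based on the prior state.
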(event `self.K2_ActivateAbility`
  (bind _montage_to_play (`self.Montage to Play`))
  (bind _asbp_player_ai (cast `/Game/SmartAIMainFolder/Blueprints/Player/BP_PlayerAI` (`self.GetAvatarActorFromActorInfo`)))
  (bind _output_get (set `self.As BP Player AI` _asbp_player_ai))
  (bind _output_get_2 (set `self.Player Controller` (`/Game/SmartAIMainFolder/Blueprints/Player/BP_PlayerAI.PlayerController` _output_get)))
  (bind _playeraicontroller (`/Game/TopDown/Blueprints/BP_TopDownController.PlayerAIController` _output_get_2))
  (bind _state (`/Game/SmartAIMainFolder/Blueprints/BP_PlayerAIController.GetCurrentPlayerState` _playeraicontroller))
  (set `self.PrevState` _state)
  (`Controller.StopMovement` _playeraicontroller)
  (bind _location (`/Game/TopDown/Blueprints/BP_TopDownController.GetLocationUnderCursor` (`self.Player Controller`)))
  (bind _result (`/Game/SmartAIMainFolder/Blueprints/Math/BFL_Math.ClampLocationInRadius` (`Actor.K2_GetActorLocation` (`self.As BP Player AI`)) _location (`self.DashMaxRadius`)))
  (set `self.Location` _result)
  (if true
    (`Actor.K2_SetActorRotation` (`self.As BP Player AI`) (`KismetMathLibrary.Conv_VectorToRotator` (- (`self.Location`) (`Actor.K2_GetActorLocation` (`self.As BP Player AI`)))) false)
    (`AbilityTask_ApplyRootMotionMoveToForce.ApplyRootMotionMoveToForce` "None" (`self.Location`) 0.2 true "MOVE_Walking" false null "SetVelocity"
      (:`then`
        (`/Engine/EditorBlueprintResources/StandardMacros.IsValid` _montage_to_play
          (:`Is Valid`
            (`AbilityTask_PlayMontageAndWait.CreatePlayMontageAndWaitProxy` "None" _montage_to_play (`self.MontageRate`)))))
      (:`OnTimedOut`
        (`self.K2_EndAbility` :!label _label)
        (switch `/Game/SmartAIMainFolder/GAS/Abilities/Player/DashWithDamage/E_DashDamageType` (`self.DamageType`)
          (:`NewEnumerator0`
            (bind _returnvalue (`|SpawnActorFromClass` "/Game/SmartAIMainFolder/Player/Blueprints/BP_HitSphereCollider.BP_HitSphereCollider_C" (`KismetMathLibrary.MakeTransform` (`self.Location`)) "AlwaysSpawn" "MultiplyWithRoot" (`self.As BP Player AI`) (`self.HitRadius`) (`self.As BP Player AI`) true 0.5 "/Script/SmartAI.SmartAICharacterWithAbilities" null :!label _label_2))
            (bind _output_get_3 (set `self.SpawnedHitCollider` _returnvalue))
            (bind _overlappingactors (`/Game/SmartAIMainFolder/Player/Blueprints/BP_HitSphereCollider.GetOverlappingActorsInSphere` _output_get_3))
            (for _array_element _overlappingactors
              (if (!= _array_element (`self.As BP Player AI`))
                (`AbilitySystemComponent.BP_ApplyGameplayEffectToTarget` :`self` (`AbilitySystemBlueprintLibrary.GetAbilitySystemComponent` (`self.As BP Player AI`)) :`GameplayEffectClass` "/Game/SmartAIMainFolder/GAS/Abilities/Player/Weapons/Bloodletter/FirstAbility/GE_Bloodletter_FirstAbility_Damage.GE_Bloodletter_FirstAbility_Damage_C" :`Target` (`AbilitySystemBlueprintLibrary.GetAbilitySystemComponent` _array_element)))))
          (:`NewEnumerator1`
            (set `self.Location` (`Actor.K2_GetActorLocation` (`self.As BP Player AI`)))
            (goto _label_2))
          (:`NewEnumerator3`
            (bind _returnvalue_2 (`|SpawnActorFromClass` "/Game/SmartAIMainFolder/Player/Blueprints/BP_HitSphereCollider.BP_HitSphereCollider_C" (`KismetMathLibrary.MakeTransform` (0.0 0.0 0.0)) "AlwaysSpawn" "MultiplyWithRoot" (`self.As BP Player AI`) (`self.HitRadius`) (`self.As BP Player AI`) true 0.5 "/Script/SmartAI.SmartAICharacterWithAbilities" null))
            (bind _output_get_4 (set `self.SpawnedHitCollider` _returnvalue_2))
            (`Actor.K2_AttachToActor` _output_get_4 (`self.As BP Player AI`) "None" "KeepRelative" "KeepRelative" "KeepRelative" true)
            (add `Actor.OnActorBeginOverlap` (`self.SpawnedHitCollider`) (delegate `OnActorBeginOverlap_Event`)))))
      (:`OnTimedOutAndDestinationReached`
        (goto _label)))
    (else
      (`self.K2_EndAbility`))))

(event `OnActorBeginOverlap_Event`
  (params (OverlappedActor :type "Actor Object Reference") (OtherActor :type "Actor Object Reference"))
  (bind _asbp_enemy_ai_base (cast `/Game/SmartAIMainFolder/Blueprints/EnemyAi/BP_EnemyAI_Base` OtherActor))
  (`AbilitySystemComponent.BP_ApplyGameplayEffectToTarget` :`self` (`AbilitySystemBlueprintLibrary.GetAbilitySystemComponent` (`self.As BP Player AI`)) :`GameplayEffectClass` "/Game/SmartAIMainFolder/GAS/Abilities/Player/Weapons/Bloodletter/FirstAbility/GE_Bloodletter_FirstAbility_Damage.GE_Bloodletter_FirstAbility_Damage_C" :`Target` (`AbilitySystemBlueprintLibrary.GetAbilitySystemComponent` _asbp_enemy_ai_base)))

(event `self.K2_OnEndAbility`
  (params (bWasCancelled :type Boolean))
  (`KismetSystemLibrary.PrintString` "parent End")
  (switch `/Game/SmartAIMainFolder/Enemy/Enums/E_AIStates` (`self.PrevState`)
    (:`NewEnumerator0`
      (`/Game/SmartAIMainFolder/Blueprints/BP_PlayerAIController.SetStateAsPassive` (`/Game/TopDown/Blueprints/BP_TopDownController.PlayerAIController` (`self.Player Controller`)) :!label _label_3))
    (:`NewEnumerator1`
      (goto _label_3))
    (:`NewEnumerator2`
      (goto _label_3))
    (:`NewEnumerator5`
      (`/Game/SmartAIMainFolder/Blueprints/BP_PlayerAIController.SetStateAsWalking` (`/Game/TopDown/Blueprints/BP_TopDownController.PlayerAIController` (`self.Player Controller`))))))