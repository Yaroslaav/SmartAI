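; GA_Teleport is a player Gameplay Ability that teleports the player character to the location under the cursor.
; After committing, it casts the avatar to BP_PlayerAI and asks its player controller for the cursor hit location.
; On a hit, a very short ApplyRootMotionMoveToForce task performs the near-instant move in Walking mode, then the ability ends.
; A missed trace ends the ability and a failed commit cancels it.
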(event `self.K2_ActivateAbility`
  (bind _returnvalue (`self.K2_CommitAbility`))
  (if _returnvalue
    (bind _asbp_player_ai (cast `/Game/SmartAIMainFolder/Blueprints/Player/BP_PlayerAI` (`self.GetAvatarActorFromActorInfo`)))
    (bind _output_get (set `self.As BP Player AI` _asbp_player_ai))
    (bind _output_get_2 (set `self.Player Controller` (`/Game/SmartAIMainFolder/Blueprints/Player/BP_PlayerAI.PlayerController` _output_get)))
    (bind (_location _hit) (`/Game/TopDown/Blueprints/BP_TopDownController.GetLocationUnderCursor` _output_get_2))
    (set `self.Location` _location)
    (if _hit
      (`AbilityTask_ApplyRootMotionMoveToForce.ApplyRootMotionMoveToForce` "None" (`self.Location`) 0.01 true "MOVE_Walking" true null "SetVelocity"
        (:`OnTimedOut`
          _)
        (:`OnTimedOutAndDestinationReached`
          _))
      (`self.K2_EndAbility`)
      (else
        (`self.K2_EndAbility`)))
    (else
      (`self.K2_CancelAbility`))))