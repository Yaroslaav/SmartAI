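; BP_ActorToPlace_Arrow is a player ability targeting indicator, filed under Teleport, that shows a circle decal and an arrow decal aimed at the cursor.
; On parameter initialization it assigns both materials, scales the circle by AOEScale and starts a fast looping timer.
; Each tick reads the top-down controller's cursor hit, turns the arrow toward it and stretches it by clamped 2D distance.
; GetClampedLocation returns the cursor point limited to Radius around the actor.
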(event `self.OnParametersInitialized`
  (bind _parameters_aoescale (break `WorldReticleParameters` (`self.Parameters`)))
  (`DecalComponent.SetDecalMaterial` (`self.Decal`) (`self.CircleDecalMaterial`))
  (`DecalComponent.SetDecalMaterial` (`self.Arrow`) (`self.ArrowDecalMaterial`))
  (bind _asbp_top_down_controller (cast `/Game/TopDown/Blueprints/BP_TopDownController` (`GameplayStatics.GetPlayerController` 0)))
  (set `self.As BP Top Down Controller` _asbp_top_down_controller)
  (`SceneComponent.SetRelativeScale3D` (`self.Decal`) _parameters_aoescale)
  (`KismetSystemLibrary.K2_SetTimerDelegate` (delegate `CustomEvent`) 0.01 true))

(event `CustomEvent`
  (bind _returnvalue (`self.K2_GetActorLocation`))
  (bind _parameters (`self.Parameters`))
  (bind (_hit _location) (`/Game/TopDown/Blueprints/BP_TopDownController.Get Location Under Cursor` (`self.As BP Top Down Controller`)))
  (bind _output_get (set `self.Location` _location))
  (if _hit
    (bind (_returnvalue_roll _returnvalue_pitch _returnvalue_yaw) (`KismetMathLibrary.BreakRotator` (`KismetMathLibrary.FindLookAtRotation` _returnvalue _output_get)))
    (`SceneComponent.K2_SetWorldLocationAndRotation` (`self.Arrow`) _returnvalue (`KismetMathLibrary.MakeRotator` _returnvalue_roll 90.0 _returnvalue_yaw) false false)
    (`SceneComponent.SetRelativeScale3D` (`self.Arrow`) (`KismetMathLibrary.MakeVector` (.x (break `WorldReticleParameters` _parameters)) (.y (break `WorldReticleParameters` _parameters)) (`KismetMathLibrary.FClamp` (`KismetMathLibrary.Vector_Distance2D` (`self.K2_GetActorLocation`) (`self.Location`)) (`self.MinArrowLength`) (.z (break `WorldReticleParameters` _parameters)))))
    (`SceneComponent.K2_SetWorldRotation` (`self.Decal`) (struct :`Pitch` 90.0) false false)))

(fn `GetClampedLocation`
  (returns (ReturnValue :type "Vector Structure"))
  (bind (_returnvalue_x _returnvalue_y) (`KismetMathLibrary.BreakVector` (`self.K2_GetActorLocation`)))
  (bind (_location_x _location_y _location_z) (`KismetMathLibrary.BreakVector` (`self.Location`)))
  (return (+ (`self.K2_GetActorLocation`) (* (`KismetMathLibrary.ClampVectorSize` (- (`KismetMathLibrary.MakeVector` _returnvalue_x _returnvalue_y _location_z) (`self.Location`)) 10.0 (`self.Radius`)) -1.0))))

(fn `UserConstructionScript`)