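; Placement indicator actor for the player's teleport ability, showing a range circle decal and a target point decal that follows the cursor.
; BeginPlay takes the radius from the circle decal's size, applies both materials and starts a fast looping timer.
; Each tick of that timer reads the top-down controller's cursor hit and moves the point there, clamped within the radius.
; GetClampedLocation offers similar vector-based clamping but is not called here.
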(event `self.ReceiveBeginPlay`
  (set `self.Radius` (.y (`DecalComponent.DecalSize` (`self.Decal`))))
  (`DecalComponent.SetDecalMaterial` (`self.Decal`) (`self.CircleDecalMaterial`))
  (`DecalComponent.SetDecalMaterial` (`self.Point`) (`self.PointDecalMaterial`))
  (bind _asbp_top_down_controller (cast `/Game/TopDown/Blueprints/BP_TopDownController` (`GameplayStatics.GetPlayerController` 0)))
  (set `self.As BP Top Down Controller` _asbp_top_down_controller)
  (`KismetSystemLibrary.K2_SetTimerDelegate` (delegate `CustomEvent`) 0.01 true))

(event `CustomEvent`
  (bind (_hit _location) (`/Game/TopDown/Blueprints/BP_TopDownController.Get Location Under Cursor` (`self.As BP Top Down Controller`)))
  (set `self.Location` _location)
  (if _hit
    (bind _result (`/Game/SmartAIMainFolder/Blueprints/Math/BFL_Math.ClampLocationInRadius` (`self.K2_GetActorLocation`) (`self.Location`) (`self.Radius`)))
    (`SceneComponent.K2_SetWorldLocationAndRotation` (`self.Point`) _result (struct :`Pitch` 90.0) false false)
    (`SceneComponent.K2_SetWorldRotation` (`self.Decal`) (struct :`Pitch` 90.0) false false)))

(fn `GetClampedLocation`
  (returns (ReturnValue :type "Vector Structure"))
  (bind (_returnvalue_x _returnvalue_y) (`KismetMathLibrary.BreakVector` (`self.K2_GetActorLocation`)))
  (bind (_location_x _location_y _location_z) (`KismetMathLibrary.BreakVector` (`self.Location`)))
  (return (+ (`self.K2_GetActorLocation`) (* (`KismetMathLibrary.ClampVectorSize` (- (`KismetMathLibrary.MakeVector` _returnvalue_x _returnvalue_y _location_z) (`self.Location`)) 10.0 (`self.Radius`)) -1.0))))

(fn `UserConstructionScript`)