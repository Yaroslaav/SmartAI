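; Gameplay Ability for the player's one-handed dagger auto attack.
; On activation it gets the target from the avatar and plays a sped-up sword slash montage while waiting for the single-target hit gameplay event.
; That event applies the dagger damage effect from the avatar's ability system to the target's, or cancels the ability if the target is invalid.
; The ability ends when the montage completes, is interrupted or is cancelled.
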(event `self.K2_ActivateAbility`
  (bind _targetactor (message `/Game/SmartAIMainFolder/Blueprints/EnemyAi/BPI_Fighter.GetTarget` (`self.GetAvatarActorFromActorInfo`)))
  (set `self.AttackTarget` _targetactor)
  (`AbilityTask_PlayMontageAndWait.CreatePlayMontageAndWaitProxy` "None" "/Game/SmartAIMainFolder/Animations/Montages/StableSwordOutwardSlash_UE_Montage.StableSwordOutwardSlash_UE_Montage" 2.5
    (:`then`
      (`AbilityTask_WaitGameplayEvent.WaitGameplayEvent` (struct :`TagName` "Event.HitTarget.Single") null
        (:`EventReceived`
          (`/Engine/EditorBlueprintResources/StandardMacros.IsValid` (`self.AttackTarget`)
            (:`Is Valid`
              (`AbilitySystemComponent.BP_ApplyGameplayEffectToTarget` :`self` (`AbilitySystemBlueprintLibrary.GetAbilitySystemComponent` (`self.GetAvatarActorFromActorInfo`)) :`GameplayEffectClass` "/Game/SmartAIMainFolder/Weapons/GE_1HDaggerDamage.GE_1HDaggerDamage_C" :`Target` (`AbilitySystemBlueprintLibrary.GetAbilitySystemComponent` (`self.AttackTarget`))))
            (:`Is Not Valid`
              (`self.K2_CancelAbility`))))))
    (:`OnCompleted`
      (`self.K2_EndAbility` :!label _label))
    (:`OnInterrupted`
      (goto _label))
    (:`OnCancelled`
      (goto _label))))

(event `self.K2_OnEndAbility`
  (params (bWasCancelled :type Boolean)))

(fn `Attack`)