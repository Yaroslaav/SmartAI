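; Gameplay ability for the preparing (targeting) stage of the player's one-handed dagger first ability.
; On activation it gets the top-down controller avatar and starts a user-confirmed WaitTargetData ground trace from its owning player, using a BP_ActorToPlace reticle within a limited range.
; Nodes to send the target data as an activate event, end the ability and commit cooldown exist but are unconnected, so they never run.
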(event `self.K2_ActivateAbility`
  (bind (_locationtype _literaltransform _sourceactor _sourcecomponent _sourceability _sourcesocketname) (break `GameplayAbilityTargetingLocationInfo` (`self.MakeTargetLocationInfoFromOwnerActor`)))
  (bind _asbp_top_down_controller (cast `/Game/TopDown/Blueprints/BP_TopDownController` (`self.GetAvatarActorFromActorInfo`)))
  (set `self.As BP Top Down Controller` _asbp_top_down_controller)
  (bind (_asynctaskproxy _data) (`AbilityTask_WaitTargetData.WaitTargetData` "None" "UserConfirmed" "/Script/GameplayAbilities.GameplayAbilityTargetActor_GroundTrace" 0.0 0.0 300.0 (struct :`Name` "NoCollision") false (make `GameplayAbilityTargetingLocationInfo` _locationtype _literaltransform (`/Game/TopDown/Blueprints/BP_TopDownController.OwningBPPlayer` (`self.As BP Top Down Controller`)) _sourcecomponent _sourceability _sourcesocketname) (struct) "/Game/SmartAIMainFolder/GAS/Abilities/Player/Teleport/BP_ActorToPlace.BP_ActorToPlace_C")))