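; Targeting-stage ability for the Bloodletter weapon, with the top-down controller as avatar and its owned player as the actor that receives the attack event.
; It cancels pending player input, then runs a user-confirmed ground-trace target selection with a reticle.
; Valid data commits the ability and sends the target to the player as a gameplay event.
; It ends if the triggered ability is inactive next tick, or commits cooldown when that ability ends.
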(event `self.K2_ActivateAbility`
  (bind _abilityeventtag (`self.AbilityEventTag`))
  (bind (_locationtype _literaltransform _sourceactor _sourcecomponent _sourceability _sourcesocketname) (break `GameplayAbilityTargetingLocationInfo` (`self.MakeTargetLocationInfoFromOwnerActor`)))
  (`KismetSystemLibrary.PrintString` "preparing")
  (bind _asbp_top_down_controller (cast `/Game/TopDown/Blueprints/BP_TopDownController` (`self.GetAvatarActorFromActorInfo`)))
  (bind _output_get (set `self.As BP Top Down Controller` _asbp_top_down_controller))
  (bind _assmart_aiability_system_component (cast `SmartAIAbilitySystemComponent` (`AbilitySystemBlueprintLibrary.GetAbilitySystemComponent` (`/Game/TopDown/Blueprints/BP_TopDownController.OwningBPPlayer` _output_get))))
  (bind _output_get_2 (set `self.PlayerASC` _assmart_aiability_system_component))
  (`AbilitySystemComponent.InputCancel` _output_get_2)
  (bind (_asynctaskproxy _data) (`AbilityTask_WaitTargetData.WaitTargetData` "None" "UserConfirmed" "/Script/GameplayAbilities.GameplayAbilityTargetActor_GroundTrace" 0.0 0.0 300.0 (struct :`Name` "NoCollision") false (make `GameplayAbilityTargetingLocationInfo` _locationtype _literaltransform (`/Game/TopDown/Blueprints/BP_TopDownController.OwningBPPlayer` (`self.As BP Top Down Controller`)) _sourcecomponent _sourceability _sourcesocketname) (make `WorldReticleParameters` (`self.AOEScale`)) (`self.Reticle Class`))
    (:`then`
      (`AsyncTaskGameplayAbilityEnded.ListenForGameplayAbilityEnd` (`self.PlayerASC`) (`self.AbilityToActivate`)
        (:`OnEnded`
          (`KismetSystemLibrary.PrintString` "End repa")
          (`self.K2_CommitAbilityCooldown` true)
          (`self.K2_EndAbility`))))
    (:`ValidData`
      (bind _returnvalue (`self.K2_CommitAbility`))
      (if _returnvalue
        (`AbilitySystemBlueprintLibrary.SendGameplayEventToActor` (`/Game/TopDown/Blueprints/BP_TopDownController.OwningBPPlayer` (`self.As BP Top Down Controller`)) _abilityeventtag (make `GameplayEventData` _abilityeventtag null null null null (struct) (struct) (struct) 0.0 _data))
        (`KismetSystemLibrary.DelayUntilNextTick`)
        (bind _spechandle (`/Game/SmartAIMainFolder/GAS/I_ASCOwner.GetGrantedAbilitySpec` (`/Game/TopDown/Blueprints/BP_TopDownController.OwningBPPlayer` (`self.As BP Top Down Controller`)) (`self.AbilityToActivate`)))
        (if (not (`SmartAIAbilitySystemComponent.IsAbilityActive` (`self.PlayerASC`) _spechandle))
          (`self.K2_EndAbility`))
        (else
          (`self.K2_CancelAbility`))))
    (:`Cancelled`
      (`self.K2_CancelAbility`))))