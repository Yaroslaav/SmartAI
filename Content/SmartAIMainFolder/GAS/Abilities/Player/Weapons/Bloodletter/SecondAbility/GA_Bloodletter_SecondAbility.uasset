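; Player gameplay ability for the Bloodletter weapon's second ability: a short dash toward the cursor that grants a timed damage buff.
; On a cursor hit, it clamps the target to a maximum radius, turns the player and dashes with root motion MoveToForce, ending when that task times out.
; As the dash starts, it plays a montage, self-applies a SetByCaller damage GameplayEffect and broadcasts it via GameplayMessageSubsystem.
; OnEndAbility sets the AI controller to Passive or Walking based on its pre-dash state.
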(event `self.K2_ActivateAbility`
  (bind _asbp_player_ai (cast `/Game/SmartAIMainFolder/Blueprints/Player/BP_PlayerAI` (`self.GetAvatarActorFromActorInfo`)))
  (bind _output_get (set `self.As BP Player AI` _asbp_player_ai))
  (bind _output_get_2 (set `self.Player Controller` (`/Game/SmartAIMainFolder/Blueprints/Player/BP_PlayerAI.PlayerController` _output_get)))
  (bind _playeraicontroller (`/Game/TopDown/Blueprints/BP_TopDownController.PlayerAIController` _output_get_2))
  (bind _state (`/Game/SmartAIMainFolder/Blueprints/BP_PlayerAIController.GetCurrentPlayerState` _playeraicontroller))
  (set `self.PrevState` _state)
  (`Controller.StopMovement` _playeraicontroller)
  (bind (_location _hit) (`/Game/TopDown/Blueprints/BP_TopDownController.GetLocationUnderCursor` (`self.Player Controller`)))
  (bind _result (`/Game/SmartAIMainFolder/Blueprints/Math/BFL_Math.ClampLocationInRadius` (`Actor.K2_GetActorLocation` (`self.As BP Player AI`)) _location (`self.DashMaxRadius`)))
  (set `self.Location` _result)
  (if _hit
    (`Actor.K2_SetActorRotation` (`self.As BP Player AI`) (`KismetMathLibrary.Conv_VectorToRotator` (- (`self.Location`) (`Actor.K2_GetActorLocation` (`self.As BP Player AI`)))) false)
    (`AbilityTask_ApplyRootMotionMoveToForce.ApplyRootMotionMoveToForce` "None" (`self.Location`) 0.21 true "MOVE_Walking" false null "SetVelocity"
      (:`then`
        (`AbilityTask_PlayMontageAndWait.CreatePlayMontageAndWaitProxy` "None" "/Game/SmartAIMainFolder/GAS/Abilities/Player/Weapons/Bloodletter/SecondAbility/AM_Bloodletter_SecondAbility_Anim.AM_Bloodletter_SecondAbility_Anim"
          (:`then`
            (bind _returnvalue (`AbilitySystemBlueprintLibrary.AssignTagSetByCallerMagnitude` (`self.MakeOutgoingGameplayEffectSpec` "/Game/SmartAIMainFolder/GAS/Abilities/Player/Weapons/Bloodletter/SecondAbility/GE_Bloodletter_SecondAbility_DamageBonus.GE_Bloodletter_SecondAbility_DamageBonus_C") (struct :`TagName` "Effect.Active.Buff.Damage.Duration") (`self.DamageBonusDuration`)))
            (bind _returnvalue_2 (`AbilitySystemBlueprintLibrary.AssignTagSetByCallerMagnitude` _returnvalue (struct :`TagName` "Effect.Active.Buff.Damage.Magnitude") (`self.DamageBonusMagnitude`)))
            (bind _returnvalue_3 (`AbilitySystemComponent.BP_ApplyGameplayEffectSpecToSelf` (`AbilitySystemBlueprintLibrary.GetAbilitySystemComponent` (`self.As BP Player AI`)) _returnvalue_2))
            (`GameplayMessageSubsystem.K2_BroadcastMessage` (subsystem `GameplayMessageSubsystem`) (struct :`TagName` "Effect.Active.Buff.Damage") (make `/Game/SmartAIMainFolder/Blueprints/S_PlayerActiveGameplayEffectInfo` (`self.As BP Player AI`) _returnvalue_3 (`self.DamageBonusMagnitude`) (`self.DamageBonusDuration`) (`self.DamageBonusEffecticon`))))))
      (:`OnTimedOut`
        (`self.K2_EndAbility` :!label _label))
      (:`OnTimedOutAndDestinationReached`
        (goto _label)))
    (else
      (`self.K2_EndAbility`))))

(event `self.K2_OnEndAbility`
  (params (bWasCancelled :type Boolean))
  (`KismetSystemLibrary.PrintString` "end ability")
  (switch `/Game/SmartAIMainFolder/Enemy/Enums/E_AIStates` (`self.PrevState`)
    (:`NewEnumerator0`
      (`/Game/SmartAIMainFolder/Blueprints/BP_PlayerAIController.SetStateAsPassive` (`/Game/TopDown/Blueprints/BP_TopDownController.PlayerAIController` (`self.Player Controller`)) :!label _label_2))
    (:`NewEnumerator1`
      (goto _label_2))
    (:`NewEnumerator2`
      (goto _label_2))
    (:`NewEnumerator5`
      (`/Game/SmartAIMainFolder/Blueprints/BP_PlayerAIController.SetStateAsWalking` (`/Game/TopDown/Blueprints/BP_TopDownController.PlayerAIController` (`self.Player Controller`))))))