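; Targeting stage of the Bloodletter weapon's first player ability, run on the top-down controller before the main ability fires.
; It shows a placement reticle through a user-confirmed ground trace from the player, then commits and sends the target data by gameplay event to trigger GA_Bloodletter_FirstAbility.
; A tick later it checks that ability is active on the player's ASC, waits for it to end, then commits cooldown and ends itself.
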(event `self.K2_ActivateAbility`
  (bind (_locationtype _literaltransform _sourceactor _sourcecomponent _sourceability _sourcesocketname) (break `GameplayAbilityTargetingLocationInfo` (`self.MakeTargetLocationInfoFromOwnerActor`)))
  (bind _asbp_top_down_controller (cast `/Game/TopDown/Blueprints/BP_TopDownController` (`self.GetAvatarActorFromActorInfo`)))
  (bind _output_get (set `self.As BP Top Down Controller` _asbp_top_down_controller))
  (bind _assmart_aiability_system_component (cast `SmartAIAbilitySystemComponent` (`AbilitySystemBlueprintLibrary.GetAbilitySystemComponent` (`/Game/TopDown/Blueprints/BP_TopDownController.OwningBPPlayer` _output_get))))
  (set `self.PlayerASC` _assmart_aiability_system_component)
  (bind (_asynctaskproxy _data) (`AbilityTask_WaitTargetData.WaitTargetData` "None" "UserConfirmed" "/Script/GameplayAbilities.GameplayAbilityTargetActor_GroundTrace" 0.0 0.0 300.0 (struct :`Name` "NoCollision") false (make `GameplayAbilityTargetingLocationInfo` _locationtype _literaltransform (`/Game/TopDown/Blueprints/BP_TopDownController.OwningBPPlayer` (`self.As BP Top Down Controller`)) _sourcecomponent _sourceability _sourcesocketname) (make `WorldReticleParameters` (128.0 400.0 400.0)) "/Game/SmartAIMainFolder/GAS/Abilities/Player/Weapons/Bloodletter/FirstAbility/BP_ActorToPlace_Bloodletter_FirstAbility.BP_ActorToPlace_Bloodletter_FirstAbility_C")
    (:`ValidData`
      (bind _returnvalue (`self.K2_CommitAbility`))
      (if _returnvalue
        (`AbilitySystemBlueprintLibrary.SendGameplayEventToActor` (`/Game/TopDown/Blueprints/BP_TopDownController.OwningBPPlayer` (`self.As BP Top Down Controller`)) (struct :`TagName` "Abilities.Weapon.FirstAbility.Activate") (make `GameplayEventData` (struct :`TagName` "Abilities.Weapon.FirstAbility.Activate") null null null null (struct) (struct) (struct) 0.0 _data))
        (`KismetSystemLibrary.DelayUntilNextTick`)
        (bind _spechandle (`/Game/SmartAIMainFolder/GAS/I_ASCOwner.GetGrantedAbilitySpec` (`/Game/TopDown/Blueprints/BP_TopDownController.OwningBPPlayer` (`self.As BP Top Down Controller`)) "/Game/SmartAIMainFolder/GAS/Abilities/Player/Weapons/Bloodletter/FirstAbility/GA_Bloodletter_FirstAbility.GA_Bloodletter_FirstAbility_C"))
        (if (`SmartAIAbilitySystemComponent.IsAbilityActive` (`self.PlayerASC`) _spechandle)
          (`AsyncTaskGameplayAbilityEnded.ListenForGameplayAbilityEnd` (`self.PlayerASC`) "/Game/SmartAIMainFolder/GAS/Abilities/Player/Weapons/Bloodletter/FirstAbility/GA_Bloodletter_FirstAbility.GA_Bloodletter_FirstAbility_C"
            (:`OnEnded`
              (`self.K2_CommitAbilityCooldown` true)
              (`self.K2_EndAbility`)))
          (else
            (`self.K2_EndAbility`)))
        (else
          (`self.K2_CancelAbility`))))
    (:`Cancelled`
      (`self.K2_CancelAbility`))))