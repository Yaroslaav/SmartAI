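; Player gameplay ability for the Bloodletter weapon's first skill: a dash toward the cursor that deals area damage on arrival.
; Activation stops AI movement, clamps the cursor hit to the dash radius, then turns the player and starts root-motion MoveToForce alongside a montage.
; When the move finishes, a spawned sphere collider gathers overlapping actors and applies a SetByCaller damage effect to each except the caster.
; Ending restores Walking or Passive from the saved state.
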(event `self.K2_ActivateAbility`
  (bind _returnvalue (`self.K2_CommitAbility`))
  (if _returnvalue
    (bind _asbp_player_ai (cast `/Game/SmartAIMainFolder/Blueprints/Player/BP_PlayerAI` (`self.GetAvatarActorFromActorInfo`)))
    (bind _output_get (set `self.As BP Player AI` _asbp_player_ai))
    (bind _output_get_2 (set `self.Player Controller` (`/Game/SmartAIMainFolder/Blueprints/Player/BP_PlayerAI.PlayerController` _output_get)))
    (bind _playeraicontroller (`/Game/TopDown/Blueprints/BP_TopDownController.PlayerAIController` _output_get_2))
    (bind _state (`/Game/SmartAIMainFolder/Blueprints/BP_PlayerAIController.GetCurrentPlayerState` _playeraicontroller))
    (set `self.PrevState` _state)
    (`Controller.StopMovement` _playeraicontroller)
    (bind (_location _hit) (`/Game/TopDown/Blueprints/BP_TopDownController.GetLocationUnderCursor` (`self.Player Controller`)))
    (bind _result (`/Game/SmartAIMainFolder/Blueprints/Math/BFL_Math.ClampLocationInRadius` (`Actor.K2_GetActorLocation` (`self.As BP Player AI`)) _location (`self.DashMaxRadius`)))
    (set `self.Location` _result)
    (if _hit
      (`Actor.K2_SetActorRotation` (`self.As BP Player AI`) (`KismetMathLibrary.Conv_VectorToRotator` (- (`self.Location`) (`Actor.K2_GetActorLocation` (`self.As BP Player AI`)))) false)
      (`AbilityTask_ApplyRootMotionMoveToForce.ApplyRootMotionMoveToForce` "None" (`self.Location`) 0.3 true "MOVE_Walking" false null "SetVelocity"
        (:`then`
          (`AbilityTask_PlayMontageAndWait.CreatePlayMontageAndWaitProxy` "None" "/Game/SmartAIMainFolder/GAS/Abilities/Player/Weapons/Bloodletter/FirstAbility/AM_Bloodletter_FirstAbility_Anim.AM_Bloodletter_FirstAbility_Anim"))
        (:`OnTimedOut`
          (`self.K2_EndAbility` :!label _label)
          (bind _returnvalue_2 (`|SpawnActorFromClass` "/Game/SmartAIMainFolder/Player/Blueprints/BP_HitSphereCollider.BP_HitSphereCollider_C" (`KismetMathLibrary.MakeTransform` (`self.Location`)) "AlwaysSpawn" "MultiplyWithRoot" (`self.As BP Player AI`) (`self.HitRadius`) (`self.As BP Player AI`) true 0.5 "/Script/SmartAI.SmartAICharacterWithAbilities" null))
          (bind _overlappingactors (`/Game/SmartAIMainFolder/Player/Blueprints/BP_HitSphereCollider.GetOverlappingActorsInSphere` _returnvalue_2))
          (for _array_element _overlappingactors
            (if (!= _array_element (`self.As BP Player AI`))
              (bind _returnvalue_3 (`AbilitySystemBlueprintLibrary.AssignTagSetByCallerMagnitude` (`self.MakeOutgoingGameplayEffectSpec` "/Game/SmartAIMainFolder/GAS/Abilities/Player/Weapons/Bloodletter/FirstAbility/GE_Bloodletter_FirstAbility_Damage.GE_Bloodletter_FirstAbility_Damage_C") (struct :`TagName` "Calculation.Damage") (`self.Damage`)))
              (`AbilitySystemComponent.BP_ApplyGameplayEffectSpecToTarget` (`AbilitySystemBlueprintLibrary.GetAbilitySystemComponent` (`self.As BP Player AI`)) _returnvalue_3 (`AbilitySystemBlueprintLibrary.GetAbilitySystemComponent` _array_element)))))
        (:`OnTimedOutAndDestinationReached`
          (goto _label)))
      (else
        (`self.K2_EndAbility`)))
    (else
      (`self.K2_CancelAbility`))))

(event `self.K2_OnEndAbility`
  (params (bWasCancelled :type Boolean))
  (switch `/Game/SmartAIMainFolder/Enemy/Enums/E_AIStates` (`self.PrevState`)
    (:`NewEnumerator0`
      (`/Game/SmartAIMainFolder/Blueprints/BP_PlayerAIController.SetStateAsPassive` (`/Game/TopDown/Blueprints/BP_TopDownController.PlayerAIController` (`self.Player Controller`)) :!label _label_2))
    (:`NewEnumerator1`
      (goto _label_2))
    (:`NewEnumerator2`
      (goto _label_2))
    (:`NewEnumerator5`
      (`/Game/SmartAIMainFolder/Blueprints/BP_PlayerAIController.SetStateAsWalking` (`/Game/TopDown/Blueprints/BP_TopDownController.PlayerAIController` (`self.Player Controller`))))))