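; Gameplay Ability for the Bloodletter weapon's player auto attack, which deals damage to the avatar's current target.
; On activation it caches the target from the avatar, plays a sword slash montage and waits for a single-target hit event.
; On that event it applies a damage effect spec to the target with a set-by-caller magnitude, or cancels if the target is invalid.
; The ability ends when the montage completes, is interrupted or is cancelled.
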(event `self.K2_ActivateAbility`
  (bind _returnvalue (`AbilitySystemBlueprintLibrary.GetAbilitySystemComponent` (`self.GetAvatarActorFromActorInfo`)))
  (bind _targetactor (message `/Game/SmartAIMainFolder/Blueprints/EnemyAi/BPI_Fighter.GetTarget` (`self.GetAvatarActorFromActorInfo`)))
  (set `self.AttackTarget` _targetactor)
  (`AbilityTask_PlayMontageAndWait.CreatePlayMontageAndWaitProxy` "None" "/Game/SmartAIMainFolder/Animations/Montages/StableSwordOutwardSlash_UE_Montage.StableSwordOutwardSlash_UE_Montage"
    (:`then`
      (`AbilityTask_WaitGameplayEvent.WaitGameplayEvent` (struct :`TagName` "Event.HitTarget.Single") null
        (:`EventReceived`
          (`/Engine/EditorBlueprintResources/StandardMacros.IsValid` (`self.AttackTarget`)
            (:`Is Valid`
              (bind _returnvalue_2 (`AbilitySystemBlueprintLibrary.AssignTagSetByCallerMagnitude` (`AbilitySystemComponent.MakeOutgoingSpec` :`self` _returnvalue :`GameplayEffectClass` "/Game/SmartAIMainFolder/GAS/Abilities/Player/Weapons/Bloodletter/AutoAttack/GE_Bloodletter_AutoAttack_Damage.GE_Bloodletter_AutoAttack_Damage_C") (struct :`TagName` "Calculation.Damage") (`self.Damage`)))
              (`AbilitySystemComponent.BP_ApplyGameplayEffectSpecToTarget` _returnvalue _returnvalue_2 (`AbilitySystemBlueprintLibrary.GetAbilitySystemComponent` (`self.AttackTarget`))))
            (:`Is Not Valid`
              (`self.K2_CancelAbility`))))))
    (:`OnCompleted`
      (`self.K2_EndAbility` :!label _label))
    (:`OnInterrupted`
      (goto _label))
    (:`OnCancelled`
      (goto _label))))

(event `self.K2_OnEndAbility`
  (params (bWasCancelled :type Boolean)))

(fn `Attack`)