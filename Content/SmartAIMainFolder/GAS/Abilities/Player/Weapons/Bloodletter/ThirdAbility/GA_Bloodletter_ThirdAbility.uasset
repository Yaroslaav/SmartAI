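; Bloodletter's third player weapon ability: a dash toward the cursor, clamped to a max radius, that damages enemies along the way.
; On commit it stops AI movement, faces the target and dashes with a root-motion MoveToForce task, playing VFX and a montage.
; A short-lived multi-hit sphere attached to the player applies SetByCaller GE damage on overlap.
; On end, it restores Walking or sets Passive based on the prior state.
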(event `self.K2_ActivateAbility`
  (bind _location (`self.Location`))
  (bind _returnvalue (`Actor.K2_GetActorLocation` (`self.As BP Player AI`)))
  (bind _returnvalue_2 (`self.K2_CommitAbility`))
  (if _returnvalue_2
    (bind _asbp_player_ai (cast `/Game/SmartAIMainFolder/Blueprints/Player/BP_PlayerAI` (`self.GetAvatarActorFromActorInfo`)))
    (bind _output_get (set `self.As BP Player AI` _asbp_player_ai))
    (bind _output_get_2 (set `self.Player Controller` (`/Game/SmartAIMainFolder/Blueprints/Player/BP_PlayerAI.PlayerController` _output_get)))
    (bind _playeraicontroller (`/Game/TopDown/Blueprints/BP_TopDownController.PlayerAIController` _output_get_2))
    (bind _state (`/Game/SmartAIMainFolder/Blueprints/BP_PlayerAIController.GetCurrentPlayerState` _playeraicontroller))
    (set `self.PrevState` _state)
    (`Controller.StopMovement` _playeraicontroller)
    (bind (_location_2 _hit) (`/Game/TopDown/Blueprints/BP_TopDownController.GetLocationUnderCursor` (`self.Player Controller`)))
    (bind _result (`/Game/SmartAIMainFolder/Blueprints/Math/BFL_Math.ClampLocationInRadius` (`Actor.K2_GetActorLocation` (`self.As BP Player AI`)) _location_2 (`self.DashMaxRadius`)))
    (set `self.Location` _result)
    (if _hit
      (`Actor.K2_SetActorRotation` (`self.As BP Player AI`) (`KismetMathLibrary.Conv_VectorToRotator` (- (`self.Location`) (`Actor.K2_GetActorLocation` (`self.As BP Player AI`)))) false)
      (`AbilityTask_ApplyRootMotionMoveToForce.ApplyRootMotionMoveToForce` "None" _location 0.21 true "MOVE_Walking" false null "SetVelocity"
        (:`then`
          (`NiagaraFunctionLibrary.SpawnSystemAtLocation` "/Game/BlinkAndDashVFX/VFX_Niagara/NS_Dash_Vampire.NS_Dash_Vampire" _returnvalue (`KismetMathLibrary.FindLookAtRotation` _returnvalue _location) (0.5 0.1 0.1))
          (bind _returnvalue_3 (`|SpawnActorFromClass` "/Game/SmartAIMainFolder/Player/Blueprints/BP_HitSphereCollider.BP_HitSphereCollider_C" (`KismetMathLibrary.MakeTransform` (0.0 0.0 0.0)) "AlwaysSpawn" "MultiplyWithRoot" (`self.As BP Player AI`) (`self.HitRadius`) (`self.As BP Player AI`) true 0.5 "/Script/SmartAI.SmartAICharacterWithAbilities" null))
          (bind _output_get_3 (set `self.SpawnedHitCollider` _returnvalue_3))
          (`Actor.K2_AttachToActor` _output_get_3 (`self.As BP Player AI`) "None" "KeepRelative" "KeepRelative" "KeepRelative" true)
          (add `Actor.OnActorBeginOverlap` (`self.SpawnedHitCollider`) (delegate `OnActorBeginOverlap_Event`))
          (`AbilityTask_PlayMontageAndWait.CreatePlayMontageAndWaitProxy` "None" "/Game/SmartAIMainFolder/GAS/Abilities/Player/Weapons/Bloodletter/SecondAbility/AM_Bloodletter_SecondAbility_Anim.AM_Bloodletter_SecondAbility_Anim"))
        (:`OnTimedOut`
          (`self.K2_EndAbility` :!label _label))
        (:`OnTimedOutAndDestinationReached`
          (goto _label)))
      (else
        (`self.K2_EndAbility`)))
    (else
      (`self.K2_CancelAbility`))))

(event `self.K2_OnEndAbility`
  (params (bWasCancelled :type Boolean))
  (switch `/Game/SmartAIMainFolder/Enemy/Enums/E_AIStates` (`self.PrevState`)
    (:`NewEnumerator0`
      (`/Game/SmartAIMainFolder/Blueprints/BP_PlayerAIController.SetStateAsPassive` (`/Game/TopDown/Blueprints/BP_TopDownController.PlayerAIController` (`self.Player Controller`)) :!label _label_2))
    (:`NewEnumerator1`
      (goto _label_2))
    (:`NewEnumerator2`
      (goto _label_2))
    (:`NewEnumerator5`
      (`/Game/SmartAIMainFolder/Blueprints/BP_PlayerAIController.SetStateAsWalking` (`/Game/TopDown/Blueprints/BP_TopDownController.PlayerAIController` (`self.Player Controller`))))))

(event `OnActorBeginOverlap_Event`
  (params (OverlappedActor :type "Actor Object Reference") (OtherActor :type "Actor Object Reference"))
  (bind _returnvalue (`AbilitySystemBlueprintLibrary.GetAbilitySystemComponent` (`self.As BP Player AI`)))
  (bind _asbp_enemy_ai_base (cast `/Game/SmartAIMainFolder/Blueprints/EnemyAi/BP_EnemyAI_Base` OtherActor))
  (bind _returnvalue_2 (`AbilitySystemBlueprintLibrary.AssignTagSetByCallerMagnitude` (`AbilitySystemComponent.MakeOutgoingSpec` :`self` _returnvalue :`GameplayEffectClass` "/Game/SmartAIMainFolder/GAS/Effects/Damage/GE_ApplyDamage.GE_ApplyDamage_C") (struct :`TagName` "Calculation.Damage") (`self.Damage`)))
  (`AbilitySystemComponent.BP_ApplyGameplayEffectSpecToTarget` _returnvalue _returnvalue_2 (`AbilitySystemBlueprintLibrary.GetAbilitySystemComponent` _asbp_enemy_ai_base)))