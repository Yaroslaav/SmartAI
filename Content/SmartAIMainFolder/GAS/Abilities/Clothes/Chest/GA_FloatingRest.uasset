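; GA_FloatingRest is a chest clothing gameplay ability that applies the GE_FloatingRest effect to its owner while playing a floating montage on the avatar's skeletal mesh.
; The effect is applied at the ability's level, and the ability ends when that effect is removed or its handle is invalid.
; Ending stops the montage and removes the effect, with EffectWasCancelled guarding against re-entry between the two paths.
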(event `self.K2_ActivateAbility`
  (bind _returnvalue (`self.GetAbilityLevel`))
  (`KismetSystemLibrary.PrintString` (`KismetStringLibrary.Conv_IntToString` _returnvalue))
  (bind _returnvalue_2 (`self.BP_ApplyGameplayEffectToOwner` "/Game/SmartAIMainFolder/GAS/Abilities/Clothes/Chest/Effects/GE_FloatingRest.GE_FloatingRest_C" _returnvalue))
  (bind _output_get (set `self.ActiveEffect` _returnvalue_2))
  (`AbilityTask_WaitGameplayEffectRemoved.WaitForGameplayEffectRemoved` _output_get
    (:`then`
      (bind _skeletalmeshcomponent (message `/Game/SmartAIMainFolder/Blueprints/I_Creature.GetSkeletalMesh` (`self.GetAvatarActorFromActorInfo`)))
      (`|PlayMontage` _skeletalmeshcomponent "/Game/SmartAIMainFolder/Animations/Montages/FloatingManny_Montage.FloatingManny_Montage"))
    (:`OnRemoved`
      (if (not (`self.EffectWasCancelled`)) :!label _label
        (`self.K2_EndAbility`)
        (set `self.EffectWasCancelled` true)))
    (:`InvalidHandle`
      (goto _label))))

(event `self.K2_OnEndAbility`
  (params (bWasCancelled :type Boolean))
  (`KismetSystemLibrary.PrintString` "End")
  (`self.MontageStop` -1.0)
  (if (not (`self.EffectWasCancelled`))
    (set `self.EffectWasCancelled` true)
    (`self.BP_RemoveGameplayEffectFromOwnerWithHandle` (`self.ActiveEffect`))))