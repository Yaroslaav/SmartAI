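; GA_Dash is a Gameplay Ability that makes its avatar actor dash forward.
; On activation it commits the ability, then runs a short constant-force root motion task along the avatar's forward vector, keeping the last root motion velocity on finish.
; The ability ends when the force finishes, or cancels if the commit fails.
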(event `self.K2_ActivateAbility`
  (bind _returnvalue (`self.K2_CommitAbility`))
  (if _returnvalue
    (`AbilityTask_ApplyRootMotionConstantForce.ApplyRootMotionConstantForce` "None" (`Actor.GetActorForwardVector` (`self.GetAvatarActorFromActorInfo`)) 1000.0 0.1 false null "MaintainLastRootMotionVelocity"
      (:`OnFinish`
        (`self.K2_EndAbility`)))
    (else
      (`self.K2_CancelAbility`))))

(event `self.K2_OnEndAbility`
  (params (bWasCancelled :type Boolean)))