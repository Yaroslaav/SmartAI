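; GA_MoveToAttackTarget is a Gameplay Ability that moves the player character toward its attack target.
; On activation it commits the ability, then casts the avatar to BP_Player and its controller to BP_TopDownController.
; It takes the target from the player's GetTargetMessage and paths to it with SimpleMoveToActor, cancelling only if the commit fails.
; The ability never calls EndAbility after starting the move.
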(event `self.K2_ActivateAbility`
  (bind _returnvalue (`self.K2_CommitAbility`))
  (if _returnvalue
    (bind _asbp_player (cast `/Game/SmartAIMainFolder/Blueprints/Player/BP_Player` (`self.GetAvatarActorFromActorInfo`)))
    (bind _output_get (set `self.BPPlayer` _asbp_player))
    (bind _asbp_top_down_controller (cast `/Game/TopDown/Blueprints/BP_TopDownController` (`Pawn.GetController` _output_get)))
    (bind _output_get_2 (set `self.PlayerController` _asbp_top_down_controller))
    (bind _targetactor (message `/Game/SmartAIMainFolder/Blueprints/EnemyAi/BPI_Fighter.GetTarget` (`self.BPPlayer`)))
    (`AIBlueprintHelperLibrary.SimpleMoveToActor` _output_get_2 _targetactor)
    (else
      (`self.K2_CancelAbility`))))