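; GA_PlayerFollowLocation is a gameplay ability that nudges the player pawn toward the destination cached on its top-down controller.
; On activation it commits, prints a debug string, casts the avatar to BP_Player and applies one movement input along the direction to BP_TopDownController's CachedDestination.
; It then ends immediately, so each activation adds a single input; a failed commit cancels the ability.
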(event `self.K2_ActivateAbility`
  (bind _returnvalue (`self.GetAvatarActorFromActorInfo`))
  (bind _returnvalue_2 (`self.K2_CommitAbility`))
  (if _returnvalue_2
    (`KismetSystemLibrary.PrintString` "Hello")
    (bind _asbp_player (cast `/Game/SmartAIMainFolder/Blueprints/Player/BP_Player` _returnvalue))
    (bind _output_get (set `self.As BP Player` _asbp_player))
    (`Pawn.AddMovementInput` _output_get (`KismetMathLibrary.GetDirectionUnitVector` (`Actor.K2_GetActorLocation` _returnvalue) (`/Game/TopDown/Blueprints/BP_TopDownController.CachedDestination` (cast `/Game/TopDown/Blueprints/BP_TopDownController` (`Pawn.GetController` (`self.As BP Player`)) :!pure true))) 1.0 false)
    (`self.K2_EndAbility`)
    (else
      (`self.K2_CancelAbility`))))

(event `self.K2_OnEndAbility`
  (params (bWasCancelled :type Boolean)))